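; Item actor that plays a spring-arm spin on pickup and can be rotated by touch while the player analyzes it.
; Two-finger swipes during the analyze state build clamped speed, which Tick applies to the arm's initial rotation and decays with FPS-adjusted damping for inertia.
; A short screen-to-world trace reports touch hits, and helpers manage sphere collision components.
; State-change and EndAnalyze events are empty hooks.
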(event `self.ReceiveBeginPlay`
  ;[1 0 0] Begin
  (set `self.CameraArmInitialRotation` (`SceneComponent.K2_GetComponentRotation` (`self.SpringArm`))))

(event `self.ReceiveTick`
  (params (DeltaSeconds :type "Float (single-precision)"))
  ;[1 0 0] Tick
  (`self.UpdateCamera`))

(event `BeginAnalyze`
  ;[1 1 1] 開始時終了時に呼ばれるイベント
  (`self.EnableCameraControl`))

(event `PlayPickup`
  ;[0 0 1] アイテムゲット時の演出
  (bind (_direction _rotatex) (`Timeline|RotateCamera` :!via `PlayFromStart`)
    (:`Update`
      (`SceneComponent.K2_SetWorldRotation` (`self.SpringArm`) (`KismetMathLibrary.MakeRotator` 0.0 0.0 _rotatex) false false))))

(event `EndAnalyze`
  ;[1 1 1] 開始時終了時に呼ばれるイベント
)

(event `BeginState`
  (params (ItemState :type "GameplayTag Structure"))
  ;[1 1 1] ステート管理系
)

(event `EndState`
  (params (ItemState :type "GameplayTag Structure"))
  ;[1 1 1] ステート管理系
)

(event `ChangeState`
  (params (NewItemState :type "GameplayTag Structure"))
  ;[1 1 1] ステート管理系
  (`self.EndState` (`self.ItemState`))
  (bind _output_get (set `self.ItemState` NewItemState))
  (`self.BeginState` _output_get))

(event `EnableCameraControl`
  ;[1 1 1] Bind & Unbind
  (bind _playercontroller (`/Game/LabyrinthCore/Blueprints/Library/Actor/BPML_Player.LbGetPlayerController`)
    (:`Succeeded`
      (add `/Game/LabyrinthCore/Blueprints/BP_PlayerController.TwoFingerSwipe` _playercontroller (delegate `EventMoveTwoFinger`)))))

(event `DisableCameraControl`
  ;[1 1 1] Bind & Unbind
  (bind _playercontroller (`/Game/LabyrinthCore/Blueprints/Library/Actor/BPML_Player.LbGetPlayerController`)
    (:`Succeeded`
      (remove `/Game/LabyrinthCore/Blueprints/BP_PlayerController.TwoFingerSwipe` _playercontroller (delegate `EventMoveTwoFinger`)))))

(event `EventMoveTwoFinger`
  ;[1 1 1] Bind & Unbind
  (`self.CalcMoveSpeed`))

(event `CalcMoveSpeed`
  (bind _returnvalue (`self.MaxSpeedX`))
  (bind _returnvalue_2 (`self.MaxSpeedY`))
  ;[0 0 1] 速度を計算
  (`/Game/LabyrinthCore/Blueprints/Library/Actor/BPML_PlayerState.LbIsPlayerState` (`/Game/LabyrinthCore/Blueprints/Const/BPCST_PlayerState.PSt_AnalyzeItem`)
    (:`true`
      (`|ExecutionSequence`
        (:`then_0`
          ;[1 1 1] タッチ座標の移動量からカメラ加速度を算出する
          (bind _playercontroller (`/Game/LabyrinthCore/Blueprints/Library/Actor/BPML_Player.LbGetPlayerController`)
            (:`Succeeded`
              (`|ExecutionSequence`
                (:`then_0`
                  (bind (_twofingertouchdeltalocation_x _twofingertouchdeltalocation_y) (`KismetMathLibrary.BreakVector` (`/Game/LabyrinthCore/Blueprints/BP_PlayerController.TwoFingerTouchDeltaLocation` _playercontroller)))
                  (set `self.AccelX` (* (`/Game/LabyrinthCore/Blueprints/Library/BPFL_Labyrinth.ApplyValueAtFPS` (* _twofingertouchdeltalocation_x (`self.AccelSpeedX`))) (`KismetMathLibrary.SelectFloat` -1.0 1.0 (`self.InverseX`)))))
                (:`then_1`
                  (set `self.AccelY` (* (`/Game/LabyrinthCore/Blueprints/Library/BPFL_Labyrinth.ApplyValueAtFPS` (* _twofingertouchdeltalocation_y (`self.AccelSpeedY`))) (`KismetMathLibrary.SelectFloat` 1.0 -1.0 (`self.InverseY`)))))))))
        (:`then_1`
          ;[1 1 1] カメラ速度に加速度を加算
          (`|ExecutionSequence`
            (:`then_0`
              (set `self.SpeedX` (`KismetMathLibrary.FClamp` (+ (`self.SpeedX`) (`self.AccelX`)) (* _returnvalue -1.0) _returnvalue)))
            (:`then_1`
              (set `self.SpeedY` (`KismetMathLibrary.FClamp` (+ (`self.SpeedY`) (`self.AccelY`)) (* _returnvalue_2 -1.0) _returnvalue_2)))))))))

(event `UpdateCamera`
  ;[0 0 1] 速度を反映
  (`|ExecutionSequence`
    (:`then_0`
      ;[1 1 1] カメラ速度をカメラ回転値に反映
      (set `self.RotateX` (+ (`self.RotateX`) (`self.SpeedX`)))
      (bind _output_get (set `self.RotateX` (mod (+ (`self.RotateX`) 360.0) 360.0)))
      (set `self.RotateX` (`KismetMathLibrary.FClamp` _output_get (`self.RotateXMin`) (`self.RotateXMax`)))
      (set `self.RotateY` (`KismetMathLibrary.FClamp` (+ (`self.RotateY`) (`self.SpeedY`)) (`self.RotateYMin`) (`self.RotateYMax`))) ; 角度制限はPlayerCameraManagerにて
    )
    (:`then_1`
      ;[1 1 1] カメラ速度を減衰させる
      (set `self.SpeedX` (`/Game/LabyrinthCore/Blueprints/Library/BPFL_Labyrinth.ApplyValueAtFPS` (* (`self.SpeedX`) (`self.DecayX`))))
      (set `self.SpeedY` (`/Game/LabyrinthCore/Blueprints/Library/BPFL_Labyrinth.ApplyValueAtFPS` (* (`self.SpeedY`) (`self.DecayY`)))))
    (:`then_2`
      ;[1 1 1] カメラ回転の反映
      (`SceneComponent.K2_SetWorldRotation` (`self.SpringArm`) (`KismetMathLibrary.MakeRotator` 0.0 (+ (.pitch (`self.CameraArmInitialRotation`)) (`self.RotateY`)) (+ (.yaw (`self.CameraArmInitialRotation`)) (`self.RotateX`))) false false))))

(fn `AddCollision`
  (params (NewItem :type "SphereComponent Object Reference (by ref)"))
  (`KismetArrayLibrary.Array_Add` (`self.SphereCollision`) NewItem))

(fn `ClearCollision`
  (bind _spherecollision (`self.SphereCollision`))
  (for _array_element _spherecollision
    (`ActorComponent.K2_DestroyComponent` _array_element))
  (`KismetArrayLibrary.Array_Clear` _spherecollision))

(fn `RaycastHitCheck`
  (params (DataTable :type "DataTable Object Reference") (SocketName :type Name))
  (returns (ReturnValue :type Boolean))
  (bind _playercontroller (`/Game/LabyrinthCore/Blueprints/Library/Actor/BPML_Player.LbGetPlayerController`)
    (:`Succeeded`
      (bind (_worldlocation _worlddirection) (`PlayerController.DeprojectScreenPositionToWorld` _playercontroller (.x (* (`/Game/LabyrinthCore/Blueprints/BP_PlayerController.TouchLocation` _playercontroller) (`WidgetLayoutLibrary.GetViewportScale`))) (.y (* (`/Game/LabyrinthCore/Blueprints/BP_PlayerController.TouchLocation` _playercontroller) (`WidgetLayoutLibrary.GetViewportScale`)))))
      (bind _outhits (`KismetSystemLibrary.LineTraceMulti` :`Start` _worldlocation :`End` (+ _worldlocation (* _worlddirection 300.0)) :`TraceChannel` "TraceTypeQuery3" :`bIgnoreSelf` false))
      (for _array_element _outhits
        (return true))
      (return false))))

(fn `UserConstructionScript`)