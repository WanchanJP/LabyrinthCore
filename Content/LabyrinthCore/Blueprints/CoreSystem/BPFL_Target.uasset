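; Blueprint function library that broadcasts objective (target) changes for main and sub targets in the game.
; Each function finds every actor implementing BPIF_Target and forwards the call as the matching interface message, so callers need no references to the receivers.
; It covers setting and completing main and sub targets by label, adding or removing sub targets, clearing all targets, and toggling their visibility.
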(fn `AddSubTarget`
  (params (Label :type Name))
  (bind _outactors (`GameplayStatics.GetAllActorsWithInterface` null "/Game/LabyrinthCore/Blueprints/CoreSystem/BPIF_Target.BPIF_Target_C"))
  (for _array_element _outactors
    (message `/Game/LabyrinthCore/Blueprints/CoreSystem/BPIF_Target.AddSubTarget` _array_element Label)))

(fn `RemoveAllTarget`
  (bind _outactors (`GameplayStatics.GetAllActorsWithInterface` null "/Game/LabyrinthCore/Blueprints/CoreSystem/BPIF_Target.BPIF_Target_C"))
  (for _array_element _outactors
    (message `/Game/LabyrinthCore/Blueprints/CoreSystem/BPIF_Target.RemoveAllTarget` _array_element)))

(fn `RemoveSubTarget`
  (params (Label :type Name))
  (bind _outactors (`GameplayStatics.GetAllActorsWithInterface` null "/Game/LabyrinthCore/Blueprints/CoreSystem/BPIF_Target.BPIF_Target_C"))
  (for _array_element _outactors
    (message `/Game/LabyrinthCore/Blueprints/CoreSystem/BPIF_Target.RemoveSubTarget` _array_element Label)))

(fn `SetMainTarget`
  (params (Label :type Name))
  (bind _outactors (`GameplayStatics.GetAllActorsWithInterface` null "/Game/LabyrinthCore/Blueprints/CoreSystem/BPIF_Target.BPIF_Target_C"))
  (for _array_element _outactors
    (message `/Game/LabyrinthCore/Blueprints/CoreSystem/BPIF_Target.SetMainTarget` _array_element Label)))

(fn `SetMainTargetComplete`
  (params (Label :type Name))
  (bind _outactors (`GameplayStatics.GetAllActorsWithInterface` null "/Game/LabyrinthCore/Blueprints/CoreSystem/BPIF_Target.BPIF_Target_C"))
  (for _array_element _outactors
    (message `/Game/LabyrinthCore/Blueprints/CoreSystem/BPIF_Target.SetMainTargetComplete` _array_element Label)))

(fn `SetSubTargetComplete`
  (params (Label :type Name))
  (bind _outactors (`GameplayStatics.GetAllActorsWithInterface` null "/Game/LabyrinthCore/Blueprints/CoreSystem/BPIF_Target.BPIF_Target_C"))
  (for _array_element _outactors
    (message `/Game/LabyrinthCore/Blueprints/CoreSystem/BPIF_Target.SetSubTargetComplete` _array_element Label)))

(fn `SetTargetVisibility`
  (params (bNewVisibility :type Boolean))
  (bind _outactors (`GameplayStatics.GetAllActorsWithInterface` null "/Game/LabyrinthCore/Blueprints/CoreSystem/BPIF_Target.BPIF_Target_C"))
  (for _array_element _outactors
    (message `/Game/LabyrinthCore/Blueprints/CoreSystem/BPIF_Target.SetTargetVisibility` _array_element bNewVisibility)))