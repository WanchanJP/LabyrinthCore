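; BP_Subtitle is the subtitle controller that shows two-text subtitles on screen.
; On BeginPlay it creates a WB_Subtitle widget and adds it to the viewport with a ZOrder from the subtitle widget priority.
; Play looks up a label in the supplied DataTable and passes that row's texts and duration to the widget.
; Stop forwards to the widget to end playback.
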(event `self.ReceiveBeginPlay`
  ;[1 0 0] Begin
  (`parent.ReceiveBeginPlay`)
  (bind _returnvalue (`|CreateWidget` "/Game/LabyrinthCore/Blueprints/WidgetBP/WB_Subtitle.WB_Subtitle_C"))
  (bind _output_get (set `self.WB_Subtitle` _returnvalue))
  (`UserWidget.AddToViewport` _output_get (`self.WidgetPriority_Subtitle`)))

(event `/Game/LabyrinthCore/Blueprints/CoreSystem/BPIF_Subtitle.Play`
  (params (Label :type Name) (DataTable :type "DataTable Object Reference"))
  (bind _wb_subtitle (`self.WB_Subtitle`))
  ;[0 0 1] 再生
  (`/Engine/EditorBlueprintResources/StandardMacros.IsValid` _wb_subtitle
    (:`Is Valid`
      (`/Engine/EditorBlueprintResources/StandardMacros.IsValid` DataTable
        (:`Is Valid`
          (bind _returnvalue (`|GetDataTableRow` DataTable Label)
            (:`then`
              (bind (_label _character _text1 _text2 _duration) (break `/Game/LabyrinthCore/Blueprints/Types/FCharacterVoice` _returnvalue))
              (`/Game/LabyrinthCore/Blueprints/WidgetBP/WB_Subtitle.Play` _wb_subtitle _text1 _text2 _duration))))))))

(event `/Game/LabyrinthCore/Blueprints/CoreSystem/BPIF_Subtitle.Stop`
  (bind _wb_subtitle (`self.WB_Subtitle`))
  ;[0 0 1] 停止
  (`/Engine/EditorBlueprintResources/StandardMacros.IsValid` _wb_subtitle
    (:`Is Valid`
      (`/Game/LabyrinthCore/Blueprints/WidgetBP/WB_Subtitle.Stop` _wb_subtitle))))

(fn `UserConstructionScript`
  (`parent.UserConstructionScript`))