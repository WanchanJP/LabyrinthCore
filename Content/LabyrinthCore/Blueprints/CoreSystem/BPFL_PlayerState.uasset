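; Blueprint function library that gives global access to the player's tag-based state for setting, adding, reading and querying it.
; Each function fetches the player character through GetPlayerCharacterBP, checks that it is valid, and forwards the call to its BPPlayerStateComponent.
; Only GetPlayerState reports failure explicitly, through a Succeeded flag.
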(fn `AddPlayerState`
  (params (Tag :type "GameplayTag Structure"))
  (bind _playercharacter (`/Game/LabyrinthCore/Blueprints/CoreSystem/BPFL_Common.GetPlayerCharacterBP` null))
  (`/Engine/EditorBlueprintResources/StandardMacros.IsValid` _playercharacter
    (:`Is Valid`
      (`/Game/LabyrinthCore/Blueprints/PlayerComponents/BP_PlayerStateComponent.AddPlayerState` (`/Game/LabyrinthCore/Blueprints/BP_PlayerCharacter.BP_PlayerStateComponent` _playercharacter) Tag)
      (return))))

(fn `GetPlayerState`
  (returns (PlayerState :type "GameplayTagContainer Structure") (bSucceeded :type Boolean))
  (bind _playercharacter (`/Game/LabyrinthCore/Blueprints/CoreSystem/BPFL_Common.GetPlayerCharacterBP` null))
  (`/Engine/EditorBlueprintResources/StandardMacros.IsValid` _playercharacter
    (:`Is Valid`
      (return (`/Game/LabyrinthCore/Blueprints/PlayerComponents/BP_PlayerStateComponent.GetPlayerState` (`/Game/LabyrinthCore/Blueprints/BP_PlayerCharacter.BP_PlayerStateComponent` _playercharacter)) true))
    (:`Is Not Valid`
      (return (struct) false))))

(fn `HasAnyPlayerState`
  (params (TagContainer :type "GameplayTagContainer Structure"))
  (returns (bSucceeded :type Boolean))
  (bind _playercharacter (`/Game/LabyrinthCore/Blueprints/CoreSystem/BPFL_Common.GetPlayerCharacterBP` null))
  (`/Engine/EditorBlueprintResources/StandardMacros.IsValid` _playercharacter
    (:`Is Valid`
      (return (`/Game/LabyrinthCore/Blueprints/PlayerComponents/BP_PlayerStateComponent.HasAnyPlayerState` (`/Game/LabyrinthCore/Blueprints/BP_PlayerCharacter.BP_PlayerStateComponent` _playercharacter) TagContainer)))))

(fn `HasPlayerState`
  (params (Tag :type "GameplayTag Structure"))
  (returns (bSucceeded :type Boolean))
  (bind _playercharacter (`/Game/LabyrinthCore/Blueprints/CoreSystem/BPFL_Common.GetPlayerCharacterBP` null))
  (`/Engine/EditorBlueprintResources/StandardMacros.IsValid` _playercharacter
    (:`Is Valid`
      (return (`/Game/LabyrinthCore/Blueprints/PlayerComponents/BP_PlayerStateComponent.HasPlayerState` (`/Game/LabyrinthCore/Blueprints/BP_PlayerCharacter.BP_PlayerStateComponent` _playercharacter) Tag)))))

(fn `IsPlayerState`
  (params (Tag :type "GameplayTag Structure"))
  (returns (ReturnValue :type Boolean))
  (bind _playercharacter (`/Game/LabyrinthCore/Blueprints/CoreSystem/BPFL_Common.GetPlayerCharacterBP` null))
  (`/Engine/EditorBlueprintResources/StandardMacros.IsValid` _playercharacter
    (:`Is Valid`
      (return (`/Game/LabyrinthCore/Blueprints/PlayerComponents/BP_PlayerStateComponent.IsPlayerState` (`/Game/LabyrinthCore/Blueprints/BP_PlayerCharacter.BP_PlayerStateComponent` _playercharacter) Tag)))))

(fn `SetPlayerState`
  (params (PlayerState :type "GameplayTagContainer Structure"))
  (bind _playercharacter (`/Game/LabyrinthCore/Blueprints/CoreSystem/BPFL_Common.GetPlayerCharacterBP` null))
  (`/Engine/EditorBlueprintResources/StandardMacros.IsValid` _playercharacter
    (:`Is Valid`
      (`/Game/LabyrinthCore/Blueprints/PlayerComponents/BP_PlayerStateComponent.SetPlayerState` (`/Game/LabyrinthCore/Blueprints/BP_PlayerCharacter.BP_PlayerStateComponent` _playercharacter) PlayerState)
      (return))))