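; BP_Target manages the on-screen objective display, showing main and sub targets identified by labels.
; On BeginPlay it creates a WB_Target widget in the viewport at the target Z-order, and removes it on EndPlay.
; Its events set, add, complete or remove targets and toggle visibility, each forwarding to the widget after a validity check.
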(event `self.ReceiveBeginPlay`
  ;[1 0 0] Begin
  (`parent.ReceiveBeginPlay`)
  (`/Game/LabyrinthCore/Blueprints/Library/Actor/BPML_Widget.LbCreateWidget` "/Game/LabyrinthCore/Blueprints/WidgetBP/WB_Target.WB_Target_C" (`self.WB_Target`) true (`/Game/LabyrinthCore/Blueprints/Const/BPCST_WidgetPriority.WPr_Target`)))

(event `self.ReceiveEndPlay`
  (params (EndPlayReason :type "EEndPlayReason Enum" :default "Destroyed"))
  (`/Game/LabyrinthCore/Blueprints/Library/Actor/BPML_Widget.LbRemoveWidget` (`self.WB_Target`)))

(event `/Game/LabyrinthCore/Blueprints/CoreSystem/BPIF_Target.SetMainTarget`
  (params (Label :type Name))
  ;[1 1 1] メインターゲットをセット
  (bind _wb_target (`self.WB_Target`)
    (:`then`
      (`/Game/LabyrinthCore/Blueprints/WidgetBP/WB_Target.SetMainTarget` _wb_target Label))
    (:`else`)))

(event `/Game/LabyrinthCore/Blueprints/CoreSystem/BPIF_Target.SetMainTargetComplete`
  (params (Label :type Name))
  ;[1 1 1] メインターゲット達成
  (bind _wb_target (`self.WB_Target`)
    (:`then`
      (`/Game/LabyrinthCore/Blueprints/WidgetBP/WB_Target.SetMainTargetComplete` _wb_target Label))
    (:`else`)))

(event `/Game/LabyrinthCore/Blueprints/CoreSystem/BPIF_Target.AddSubTarget`
  (params (Label :type Name))
  (bind _wb_target (`self.WB_Target`)
    (:`then`
      (`/Game/LabyrinthCore/Blueprints/WidgetBP/WB_Target.AddSubTarget` _wb_target Label))
    (:`else`)))

(event `/Game/LabyrinthCore/Blueprints/CoreSystem/BPIF_Target.SetSubTargetComplete`
  (params (Label :type Name))
  (bind _wb_target (`self.WB_Target`)
    (:`then`
      (`/Game/LabyrinthCore/Blueprints/WidgetBP/WB_Target.SetSubTargetComplete` _wb_target Label))
    (:`else`)))

(event `/Game/LabyrinthCore/Blueprints/CoreSystem/BPIF_Target.RemoveAllTarget`
  (bind _wb_target (`self.WB_Target`)
    (:`then`
      (`/Game/LabyrinthCore/Blueprints/WidgetBP/WB_Target.RemoveAllTarget` _wb_target))
    (:`else`)))

(event `/Game/LabyrinthCore/Blueprints/CoreSystem/BPIF_Target.RemoveSubTarget`
  (params (Label :type Name))
  (bind _wb_target (`self.WB_Target`)
    (:`then`
      (`/Game/LabyrinthCore/Blueprints/WidgetBP/WB_Target.RemoveSubTarget` _wb_target Label))
    (:`else`)))

(event `/Game/LabyrinthCore/Blueprints/CoreSystem/BPIF_Target.SetTargetVisibility`
  (params (bNewVisibility :type Boolean))
  ;[1 1 1] 表示/非表示 切り替え
  (bind _wb_target (`self.WB_Target`)
    (:`then`
      (`/Game/LabyrinthCore/Blueprints/WidgetBP/WB_Target.SetTargetVisibility` _wb_target bNewVisibility))
    (:`else`)))

(fn `UserConstructionScript`)