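; Common Blueprint function library for the Labyrinth core system, giving shortcuts to the project's main framework objects.
; Getters validate and cast the index 0 player character, player controller and game state to their BP classes.
; RemoteEvent prefixes the given event name with "CE" and executes it as a console command through that controller, triggering custom events by name.
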(fn `GetGameStateBP`
  (returns (GameState :type "/Game/LabyrinthCore/Blueprints/BP_GameState Object Reference"))
  (bind _returnvalue (`GameplayStatics.GetGameState` null))
  (`/Engine/EditorBlueprintResources/StandardMacros.IsValid` _returnvalue
    (:`Is Valid`
      (bind _asbp_game_state (cast `/Game/LabyrinthCore/Blueprints/BP_GameState` _returnvalue))
      (return _asbp_game_state))))

(fn `GetPlayerCharacterBP`
  (returns (PlayerCharacter :type "/Game/LabyrinthCore/Blueprints/BP_PlayerCharacter Object Reference"))
  (bind _returnvalue (`GameplayStatics.GetPlayerCharacter` null))
  (`/Engine/EditorBlueprintResources/StandardMacros.IsValid` _returnvalue
    (:`Is Valid`
      (bind _asbp_player_character (cast `/Game/LabyrinthCore/Blueprints/BP_PlayerCharacter` _returnvalue))
      (return _asbp_player_character))))

(fn `GetPlayerControllerBP`
  (returns (PlayerController :type "/Game/LabyrinthCore/Blueprints/BP_PlayerController Object Reference"))
  (bind _returnvalue (`GameplayStatics.GetPlayerController` null))
  (`/Engine/EditorBlueprintResources/StandardMacros.IsValid` _returnvalue
    (:`Is Valid`
      (bind _asbp_player_controller (cast `/Game/LabyrinthCore/Blueprints/BP_PlayerController` _returnvalue))
      (return _asbp_player_controller))))

(fn `RemoteEvent`
  (params (RemoteEvent :type Name))
  (bind _playercontroller (`self.GetPlayerControllerBP` null))
  (`/Engine/EditorBlueprintResources/StandardMacros.IsValid` _playercontroller
    (:`Is Valid`
      (`KismetSystemLibrary.ExecuteConsoleCommand` null (`KismetStringLibrary.Concat_StrStr` "CE " (`KismetStringLibrary.Conv_NameToString` RemoteEvent)) _playercontroller))))