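; Level streaming manager that loads, unloads and plays sublevels, individually or grouped into named areas.
; A JSON file's "Labyrinth" array flags which sublevels each area needs, driving area load, unload and loaded-state checks.
; Batch macros use manual index loops instead of ForEachLoop, so each latent streaming call completes before the next.
; Play requests load missing levels, poll visibility on a looping timer, then fire a "<LevelName>_Play" remote event.
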(event `/Game/LabyrinthCore/Blueprints/CoreSystem/BPIF_LevelStreaming.LoadStreamLevel`
  (params (LevelName :type Name))
  ;[1 1 1] サブレベルをロードする
  (if (!= LevelName "None")
    (`GameplayStatics.LoadStreamLevel` LevelName true)
    (`KismetArrayLibrary.Array_Add` (`self.LoadedLevelNames`) LevelName)))

(event `/Game/LabyrinthCore/Blueprints/CoreSystem/BPIF_LevelStreaming.UnloadStreamLevel`
  (params (LevelName :type Name))
  ;[1 1 1] サブレベルをアンロードする
  (if (!= LevelName "None")
    (`GameplayStatics.UnloadStreamLevel` LevelName)
    (`KismetArrayLibrary.Array_RemoveItem` (`self.LoadedLevelNames`) LevelName)))

(event `/Game/LabyrinthCore/Blueprints/CoreSystem/BPIF_LevelStreaming.PlayStreamLevel`
  (params (LevelName :type Name))
  ;[1 1 1] サブレベルを再生する
  (if (!= LevelName "None")
    (if (not (>= (`KismetArrayLibrary.Array_Find` (`self.PlayingLevelNames`) LevelName) 0))
      (if (not (>= (`KismetArrayLibrary.Array_Find` (`self.LoadedLevelNames`) LevelName) 0))
        (`/Game/LabyrinthCore/Blueprints/CoreSystem/BPIF_LevelStreaming.LoadStreamLevel` LevelName))
      (set `self.PlayRequestLevelName` LevelName)
      (bind _returnvalue (`KismetSystemLibrary.K2_SetTimerDelegate` (delegate `Play`) 0.1 true)))))

(event `StopTimer`
  ;[1 1 1] サブレベルを再生する
  (`KismetSystemLibrary.K2_ClearAndInvalidateTimerHandle` (stale `/Game/LabyrinthCore/Blueprints/CoreSystem/BPIF_LevelStreaming.PlayStreamLevel` _returnvalue))
  (set `self.PlayRequestLevelName` "None"))

(event `Play`
  (bind _playrequestlevelname (`self.PlayRequestLevelName`))
  ;[1 1 1] サブレベルを再生する
  (bind _returnvalue (`/Game/LabyrinthCore/Blueprints/CoreSystem/BPIF_LevelStreaming.IsLoadedStreamLevel` _playrequestlevelname))
  (if _returnvalue
    (`/Game/LabyrinthCore/Blueprints/Library/Actor/BPML_RemoteEvent.LbRemoteEvent` (`/Game/LabyrinthCore/Blueprints/Library/BPFL_Labyrinth.AppendName` _playrequestlevelname "_Play"))
    (`KismetArrayLibrary.Array_Add` (`self.PlayingLevelNames`) _playrequestlevelname)
    (`self.StopTimer`)))

(event `/Game/LabyrinthCore/Blueprints/CoreSystem/BPIF_LevelStreaming.SetupAreaLevels`
  (params (FilePath :type String))
  ;[1 1 1] エリアのセットアップ
  (set `self.AreaJsonData` null)
  (bind _output_get (set `self.AreaJsonData` (`JsonFieldData.Create`)))
  (`JsonFieldData.FromFile` _output_get FilePath))

(event `/Game/LabyrinthCore/Blueprints/CoreSystem/BPIF_LevelStreaming.LoadAreaLevels`
  (params (AreaName :type String))
  ;[1 1 1] エリアを読み込む
  (`KismetArrayLibrary.Array_Clear` (`self.LoadedAreaNames`))
  (`KismetArrayLibrary.Array_Clear` (`self.UnloadedAreaNames`))
  (bind (_sublevel _bload) (`self.IsNeedLoadSubLevels` AreaName)
    (:`Loop`
      (if _bload
        (`KismetArrayLibrary.Array_Add` (`self.LoadedAreaNames`) _sublevel)
        (else
          (`KismetArrayLibrary.Array_Add` (`self.UnloadedAreaNames`) _sublevel))))
    (:`Completed`
      (`self.LoadStreamLevels` (`self.LoadedAreaNames`))
      (`self.UnloadStreamLevels` (`self.UnloadedAreaNames`)))))

(event `/Game/LabyrinthCore/Blueprints/CoreSystem/BPIF_LevelStreaming.UnloadAreaLevels`
  (bind _areajsondata (`self.AreaJsonData`))
  (bind (_success _returnvalue) (`JsonFieldData.GetObjectArray` _areajsondata "Labyrinth"))
  ;[1 1 1] エリアを破棄する
  (`KismetArrayLibrary.Array_Clear` (`self.LoadedAreaNames`))
  (`KismetArrayLibrary.Array_Clear` (`self.UnloadedAreaNames`))
  (`/Engine/EditorBlueprintResources/StandardMacros.IsValid` _areajsondata
    (:`Is Valid`
      (if _success
        (for _array_element _returnvalue
          (for _array_element_2 (`JsonFieldData.GetObjectKeys` _array_element)
            (`KismetArrayLibrary.Array_AddUnique` (`self.UnloadedAreaNames`) _array_element_2)))
        (`self.UnloadStreamLevels` (`self.UnloadedAreaNames`))))))

(fn `IsLoadedAreaLevels`
  (params (AreaName :type String))
  (returns (ReturnValue :type Boolean))
  (bind (_sublevel _bload) (`self.IsNeedLoadSubLevels` AreaName)
    (:`Loop`
      (if _bload
        (bind _returnvalue (`/Game/LabyrinthCore/Blueprints/CoreSystem/BPIF_LevelStreaming.IsLoadedStreamLevel` (`KismetStringLibrary.Conv_StringToName` _sublevel)))
        (if (not _returnvalue)
          (return false))))
    (:`Completed`
      (return true))))

(fn `IsLoadedStreamLevel`
  (params (LevelName :type Name))
  (returns (ReturnValue :type Boolean))
  (bind _returnvalue (`GameplayStatics.GetStreamingLevel` LevelName))
  (if (!= LevelName "None")
    (`/Engine/EditorBlueprintResources/StandardMacros.IsValid` _returnvalue
      (:`Is Valid`
        (return (`LevelStreaming.IsLevelVisible` _returnvalue)))
      (:`Is Not Valid`
        (return false)))))

(fn `UserConstructionScript`)