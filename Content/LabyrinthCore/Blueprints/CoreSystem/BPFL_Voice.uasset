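; Blueprint function library that starts and stops voice lines, with optional subtitles.
; PlayVoice finds every actor implementing BPIF_Voice and sends it PlayMessage with a label and DataTable; StopVoice sends StopMessage the same way.
; When the Subtitle flag is set, both functions also broadcast the same message to every BPIF_Subtitle actor.
; Actors are looked up by interface on each call, so the library needs no direct references to them.
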(fn `PlayVoice`
  (params (Label :type Name) (DataTable :type "DataTable Object Reference") (bSubtitle :type Boolean))
  (`|ExecutionSequence`
    (:`then_0`
      (bind _outactors (`GameplayStatics.GetAllActorsWithInterface` null "/Game/LabyrinthCore/Blueprints/CoreSystem/BPIF_Voice.BPIF_Voice_C"))
      (for _array_element _outactors
        (message `/Game/LabyrinthCore/Blueprints/CoreSystem/BPIF_Voice.Play` _array_element Label DataTable)))
    (:`then_1`
      (if bSubtitle
        (bind _outactors_2 (`GameplayStatics.GetAllActorsWithInterface` null "/Game/LabyrinthCore/Blueprints/CoreSystem/BPIF_Subtitle.BPIF_Subtitle_C"))
        (for _array_element_2 _outactors_2
          (message `/Game/LabyrinthCore/Blueprints/CoreSystem/BPIF_Subtitle.Play` _array_element_2 Label DataTable))))))

(fn `StopVoice`
  (params (bSubtitle :type Boolean))
  (`|ExecutionSequence`
    (:`then_0`
      (bind _outactors (`GameplayStatics.GetAllActorsWithInterface` null "/Game/LabyrinthCore/Blueprints/CoreSystem/BPIF_Voice.BPIF_Voice_C"))
      (for _array_element _outactors
        (message `/Game/LabyrinthCore/Blueprints/CoreSystem/BPIF_Voice.Stop` _array_element)))
    (:`then_1`
      (if bSubtitle
        (bind _outactors_2 (`GameplayStatics.GetAllActorsWithInterface` null "/Game/LabyrinthCore/Blueprints/CoreSystem/BPIF_Subtitle.BPIF_Subtitle_C"))
        (for _array_element_2 _outactors_2
          (message `/Game/LabyrinthCore/Blueprints/CoreSystem/BPIF_Subtitle.Stop` _array_element_2))))))