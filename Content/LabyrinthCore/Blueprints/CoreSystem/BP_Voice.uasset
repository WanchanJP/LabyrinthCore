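; BP_Voice plays voice sounds by label from a supplied DataTable, one at a time.
; Play first stops any current sound, then looks up the row, creates a 2D sound from its SoundCue, stores it as PlayingSound and starts it.
; Stop halts the stored sound if it is valid and still playing.
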(event `self.Play`
  (params (Label :type Name) (DataTable :type "DataTable Object Reference"))
  ;[0 0 1] 再生
  (`self.Stop`) ; 再生中かもしれないので停止を呼ぶ
  (`/Engine/EditorBlueprintResources/StandardMacros.IsValid` DataTable
    (:`Is Valid`
      (bind _returnvalue (`|GetDataTableRow` DataTable Label)
        (:`then`
          (bind _returnvalue_2 (`GameplayStatics.CreateSound2D` (`.SoundCue_15_A37B9B984CF13DD30BA587B4BE3FDFCF` (break `/Game/LabyrinthCore/Blueprints/Types/FCharacterVoice` _returnvalue)) 1.0 1.0 0.0 null))
          (bind _output_get (set `self.PlayingSound` _returnvalue_2))
          (`AudioComponent.Play` _output_get 0.0))))))

(event `self.Stop`
  (bind _playingsound (`self.PlayingSound`))
  ;[0 0 1] 停止
  (`/Engine/EditorBlueprintResources/StandardMacros.IsValid` _playingsound
    (:`Is Valid`
      (if (`AudioComponent.IsPlaying` _playingsound)
        (`AudioComponent.Stop` _playingsound)))))

(fn `UserConstructionScript`)