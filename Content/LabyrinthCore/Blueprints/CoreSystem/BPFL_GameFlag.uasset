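; Blueprint function library for setting and querying game flags stored as gameplay tags.
; Flags live in the GameFlag tag container on the game instance, which every function checks for validity first.
; It offers adding a flag plus exact-match checks for a single, all or any of the given tags, with no function to remove one.
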(fn `HasAllGameFlag`
  (params (GameFlags :type "GameplayTagContainer Structure (by ref)"))
  (returns (ReturnValue :type Boolean))
  (bind _gameinstance (`/Game/LabyrinthCore/Blueprints/CoreSystem/BPFL_GameInstance.GetGameInstanceBP` null))
  (`/Engine/EditorBlueprintResources/StandardMacros.IsValid` _gameinstance
    (:`Is Valid`
      (return (`BlueprintGameplayTagLibrary.HasAllTags` (`/Game/LabyrinthCore/Blueprints/BP_GameInstance.GameFlag` _gameinstance) GameFlags true)))))

(fn `HasAnyGameFlag`
  (params (GameFlags :type "GameplayTagContainer Structure (by ref)"))
  (returns (ReturnValue :type Boolean))
  (bind _gameinstance (`/Game/LabyrinthCore/Blueprints/CoreSystem/BPFL_GameInstance.GetGameInstanceBP` null))
  (`/Engine/EditorBlueprintResources/StandardMacros.IsValid` _gameinstance
    (:`Is Valid`
      (return (`BlueprintGameplayTagLibrary.HasAnyTags` (`/Game/LabyrinthCore/Blueprints/BP_GameInstance.GameFlag` _gameinstance) GameFlags true)))))

(fn `IsGameFlag`
  (params (Tag :type "GameplayTag Structure"))
  (returns (ReturnValue :type Boolean))
  (bind _gameinstance (`/Game/LabyrinthCore/Blueprints/CoreSystem/BPFL_GameInstance.GetGameInstanceBP` null))
  (`/Engine/EditorBlueprintResources/StandardMacros.IsValid` _gameinstance
    (:`Is Valid`
      (return (`BlueprintGameplayTagLibrary.HasTag` (`/Game/LabyrinthCore/Blueprints/BP_GameInstance.GameFlag` _gameinstance) Tag true)))))

(fn `SetGameFlag`
  (params (GameFlag :type "GameplayTag Structure"))
  (bind _gameinstance (`/Game/LabyrinthCore/Blueprints/CoreSystem/BPFL_GameInstance.GetGameInstanceBP` null))
  (`/Engine/EditorBlueprintResources/StandardMacros.IsValid` _gameinstance
    (:`Is Valid`
      (`BlueprintGameplayTagLibrary.AddGameplayTag` (`/Game/LabyrinthCore/Blueprints/BP_GameInstance.GameFlag` _gameinstance) GameFlag))))