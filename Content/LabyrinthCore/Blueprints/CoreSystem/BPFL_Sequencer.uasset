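; Blueprint function library that gives global playback control over sequencer actors.
; Each function gathers all actors implementing BPIF_Sequencer and sends the matching interface message: play with a given sequence player, stop, pause, fast-forward, rewind, or set the transform origin.
; The transform origin getter returns the value from the first implementing actor it finds.
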(fn `FastForwardSequencer`
  (bind _outactors (`GameplayStatics.GetAllActorsWithInterface` null "/Game/LabyrinthCore/Blueprints/CoreSystem/BPIF_Sequencer.BPIF_Sequencer_C"))
  (for _array_element _outactors
    (message `/Game/LabyrinthCore/Blueprints/CoreSystem/BPIF_Sequencer.FastForward` _array_element)))

(fn `GetActorTransformOrigin`
  (returns (Transform :type "Transform Structure"))
  (bind _outactors (`GameplayStatics.GetAllActorsWithInterface` null "/Game/LabyrinthCore/Blueprints/CoreSystem/BPIF_Sequencer.BPIF_Sequencer_C"))
  (for _array_element _outactors
    (bind _transform (message `/Game/LabyrinthCore/Blueprints/CoreSystem/BPIF_Sequencer.GetActorTransformOrigin` _array_element))
    (return _transform)))

(fn `PauseSequencer`
  (bind _outactors (`GameplayStatics.GetAllActorsWithInterface` null "/Game/LabyrinthCore/Blueprints/CoreSystem/BPIF_Sequencer.BPIF_Sequencer_C"))
  (for _array_element _outactors
    (message `/Game/LabyrinthCore/Blueprints/CoreSystem/BPIF_Sequencer.Pause` _array_element)))

(fn `Play Sequencer`
  (params (SequencePlayer :type "LevelSequencePlayer Object Reference"))
  (bind _outactors (`GameplayStatics.GetAllActorsWithInterface` null "/Game/LabyrinthCore/Blueprints/CoreSystem/BPIF_Sequencer.BPIF_Sequencer_C"))
  (for _array_element _outactors
    (message `/Game/LabyrinthCore/Blueprints/CoreSystem/BPIF_Sequencer.Play` _array_element SequencePlayer)))

(fn `RewindSequencer`
  (bind _outactors (`GameplayStatics.GetAllActorsWithInterface` null "/Game/LabyrinthCore/Blueprints/CoreSystem/BPIF_Sequencer.BPIF_Sequencer_C"))
  (for _array_element _outactors
    (message `/Game/LabyrinthCore/Blueprints/CoreSystem/BPIF_Sequencer.Rewind` _array_element)))

(fn `SetActorTransformOrigin`
  (params (Transform :type "Transform Structure"))
  (bind _outactors (`GameplayStatics.GetAllActorsWithInterface` null "/Game/LabyrinthCore/Blueprints/CoreSystem/BPIF_Sequencer.BPIF_Sequencer_C"))
  (for _array_element _outactors
    (message `/Game/LabyrinthCore/Blueprints/CoreSystem/BPIF_Sequencer.SetActorTransformOrigin` _array_element Transform)))

(fn `StopSequencer`
  (bind _outactors (`GameplayStatics.GetAllActorsWithInterface` null "/Game/LabyrinthCore/Blueprints/CoreSystem/BPIF_Sequencer.BPIF_Sequencer_C"))
  (for _array_element _outactors
    (message `/Game/LabyrinthCore/Blueprints/CoreSystem/BPIF_Sequencer.Stop` _array_element)))