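; Blueprint function library that serves as a global access point for level streaming by individual level name or by area.
; Each function finds all actors implementing BPIF_LevelStreaming and forwards a matching interface message to load, unload, play, query or set up levels.
; The loaded-state queries return the answer of the first actor found, while the other calls reach every implementer.
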(fn `IsLoadedAreaLevels`
  (params (AreaName :type String))
  (returns (ReturnValue :type Boolean))
  (bind _outactors (`GameplayStatics.GetAllActorsWithInterface` null "/Game/LabyrinthCore/Blueprints/CoreSystem/BPIF_LevelStreaming.BPIF_LevelStreaming_C"))
  (for _array_element _outactors
    (bind _returnvalue (message `/Game/LabyrinthCore/Blueprints/CoreSystem/BPIF_LevelStreaming.IsLoadedAreaLevels` _array_element AreaName))
    (return _returnvalue)))

(fn `IsLoadedStreamLevel`
  (params (LevelName :type Name))
  (returns (ReturnValue :type Boolean))
  (bind _outactors (`GameplayStatics.GetAllActorsWithInterface` null "/Game/LabyrinthCore/Blueprints/CoreSystem/BPIF_LevelStreaming.BPIF_LevelStreaming_C"))
  (for _array_element _outactors
    (bind _returnvalue (message `/Game/LabyrinthCore/Blueprints/CoreSystem/BPIF_LevelStreaming.IsLoadedStreamLevel` _array_element LevelName))
    (return _returnvalue)))

(fn `LoadAreaLevels`
  (params (AreaName :type String))
  (bind _outactors (`GameplayStatics.GetAllActorsWithInterface` null "/Game/LabyrinthCore/Blueprints/CoreSystem/BPIF_LevelStreaming.BPIF_LevelStreaming_C"))
  (for _array_element _outactors
    (message `/Game/LabyrinthCore/Blueprints/CoreSystem/BPIF_LevelStreaming.LoadAreaLevels` _array_element AreaName)))

(fn `LoadStreamLevel`
  (params (LevelName :type Name))
  (bind _outactors (`GameplayStatics.GetAllActorsWithInterface` null "/Game/LabyrinthCore/Blueprints/CoreSystem/BPIF_LevelStreaming.BPIF_LevelStreaming_C"))
  (for _array_element _outactors
    (message `/Game/LabyrinthCore/Blueprints/CoreSystem/BPIF_LevelStreaming.LoadStreamLevel` _array_element LevelName)))

(fn `PlayStreamLevel`
  (params (LevelName :type Name))
  (bind _outactors (`GameplayStatics.GetAllActorsWithInterface` null "/Game/LabyrinthCore/Blueprints/CoreSystem/BPIF_LevelStreaming.BPIF_LevelStreaming_C"))
  (for _array_element _outactors
    (message `/Game/LabyrinthCore/Blueprints/CoreSystem/BPIF_LevelStreaming.PlayStreamLevel` _array_element LevelName)))

(fn `SetupAreaLevels`
  (params (FilePath :type String))
  (bind _outactors (`GameplayStatics.GetAllActorsWithInterface` null "/Game/LabyrinthCore/Blueprints/CoreSystem/BPIF_LevelStreaming.BPIF_LevelStreaming_C"))
  (for _array_element _outactors
    (message `/Game/LabyrinthCore/Blueprints/CoreSystem/BPIF_LevelStreaming.SetupAreaLevels` _array_element FilePath)))

(fn `UnloadAreaLevels`
  (bind _outactors (`GameplayStatics.GetAllActorsWithInterface` null "/Game/LabyrinthCore/Blueprints/CoreSystem/BPIF_LevelStreaming.BPIF_LevelStreaming_C"))
  (for _array_element _outactors
    (message `/Game/LabyrinthCore/Blueprints/CoreSystem/BPIF_LevelStreaming.UnloadAreaLevels` _array_element)))

(fn `UnloadStreamLevel`
  (params (LevelName :type Name))
  (bind _outactors (`GameplayStatics.GetAllActorsWithInterface` null "/Game/LabyrinthCore/Blueprints/CoreSystem/BPIF_LevelStreaming.BPIF_LevelStreaming_C"))
  (for _array_element _outactors
    (message `/Game/LabyrinthCore/Blueprints/CoreSystem/BPIF_LevelStreaming.UnloadStreamLevel` _array_element LevelName)))