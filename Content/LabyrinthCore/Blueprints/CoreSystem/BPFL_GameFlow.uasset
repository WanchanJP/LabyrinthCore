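; Blueprint function library that loads, plays, unloads and queries named gameflows, with loaded and current names stored on the game state.
; Load, Play and Unload fire remote events built by appending _Begin, _Play or _End to the name; Play also sets the current gameflow.
; Begin and End completion functions set or clear the stored names.
; IsActiveLoadedGameflow returns true when a loaded gameflow differs from the current one.
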(fn `GameflowBeginCompleted`
  (params (GameflowName :type Name))
  (bind _gamestate (`/Game/LabyrinthCore/Blueprints/CoreSystem/BPFL_Common.GetGameStateBP` null))
  (`/Engine/EditorBlueprintResources/StandardMacros.IsValid` _gamestate
    (:`Is Valid`
      (`/Game/LabyrinthCore/Blueprints/BP_GameState.SetLoadedGameflow` _gamestate GameflowName))))

(fn `GameflowEndCompleted`
  (params (GameflowName :type Name))
  (locals (GameState :type "/Game/LabyrinthCore/Blueprints/BP_GameState Object Reference"))
  (bind _gamestate (`/Game/LabyrinthCore/Blueprints/CoreSystem/BPFL_Common.GetGameStateBP` null))
  (`/Engine/EditorBlueprintResources/StandardMacros.IsValid` _gamestate
    (:`Is Valid`
      (set `local.GameState` _gamestate)
      (`|ExecutionSequence`
        (:`then_0`
          (if (== (`.LoadedGameflow` (`/Game/LabyrinthCore/Blueprints/BP_GameState.GetLoadedGameflow` (`local.GameState`))) (`local.GameflowName`))
            (`/Game/LabyrinthCore/Blueprints/BP_GameState.SetLoadedGameflow` (`local.GameState`) "None")))
        (:`then_1`
          (if (== (`.CurrentGameflow` (`/Game/LabyrinthCore/Blueprints/BP_GameState.GetCurrentGameflow` (`local.GameState`))) (`local.GameflowName`))
            (`/Game/LabyrinthCore/Blueprints/BP_GameState.SetCurrentGameflow` (`local.GameState`) "None")))))))

(fn `GetCurrentGameflow`
  (returns (bSucceeded :type Boolean) (CurrentGameflow :type Name))
  (bind _gamestate (`/Game/LabyrinthCore/Blueprints/CoreSystem/BPFL_Common.GetGameStateBP` null))
  (bind (_bsucceeded _currentgameflow) (`/Game/LabyrinthCore/Blueprints/BP_GameState.GetCurrentGameflow` _gamestate))
  (`/Engine/EditorBlueprintResources/StandardMacros.IsValid` _gamestate
    (:`Is Valid`
      (return _bsucceeded _currentgameflow))
    (:`Is Not Valid`
      (return false "None"))))

(fn `GetLoadedGameflow`
  (returns (bSucceeded :type Boolean) (LoadedGameflow :type Name))
  (bind _gamestate (`/Game/LabyrinthCore/Blueprints/CoreSystem/BPFL_Common.GetGameStateBP` null))
  (bind (_bsucceeded _loadedgameflow) (`/Game/LabyrinthCore/Blueprints/BP_GameState.GetLoadedGameflow` _gamestate))
  (`/Engine/EditorBlueprintResources/StandardMacros.IsValid` _gamestate
    (:`Is Valid`
      (return _bsucceeded _loadedgameflow))
    (:`Is Not Valid`
      (return false "None"))))

(fn `IsActiveLoadedGameflow`
  (returns (bSucceeded :type Boolean) (ReturnValue :type Boolean))
  (bind _gamestate (`/Game/LabyrinthCore/Blueprints/CoreSystem/BPFL_Common.GetGameStateBP` null))
  (bind (_bsucceeded _loadedgameflow) (`/Game/LabyrinthCore/Blueprints/BP_GameState.GetLoadedGameflow` _gamestate))
  (bind (_bsucceeded_2 _currentgameflow) (`/Game/LabyrinthCore/Blueprints/BP_GameState.GetCurrentGameflow` _gamestate))
  (`/Engine/EditorBlueprintResources/StandardMacros.IsValid` _gamestate
    (:`Is Valid`
      (if (!= _loadedgameflow "None")
        (return (and _bsucceeded _bsucceeded_2) (!= _loadedgameflow _currentgameflow))
        (else
          (return false false) ; LoadedGameflowが空なら抜ける
        )))
    (:`Is Not Valid`
      (return false false))))

(fn `IsCurrentGameflow`
  (params (GameflowName :type Name))
  (returns (bSucceeded :type Boolean) (ReturnValue :type Boolean))
  (bind _gamestate (`/Game/LabyrinthCore/Blueprints/CoreSystem/BPFL_Common.GetGameStateBP` null))
  (bind (_bsucceeded _currentgameflow) (`/Game/LabyrinthCore/Blueprints/BP_GameState.GetCurrentGameflow` _gamestate))
  (`/Engine/EditorBlueprintResources/StandardMacros.IsValid` _gamestate
    (:`Is Valid`
      (return _bsucceeded (== _currentgameflow GameflowName)))
    (:`Is Not Valid`
      (return false false))))

(fn `IsLoadedGameflow`
  (params (GameflowName :type Name))
  (returns (bSucceeded :type Boolean) (ReturnValue :type Boolean))
  (bind _gamestate (`/Game/LabyrinthCore/Blueprints/CoreSystem/BPFL_Common.GetGameStateBP` null))
  (bind (_bsucceeded _loadedgameflow) (`/Game/LabyrinthCore/Blueprints/BP_GameState.GetLoadedGameflow` _gamestate))
  (`/Engine/EditorBlueprintResources/StandardMacros.IsValid` _gamestate
    (:`Is Valid`
      (return _bsucceeded (== _loadedgameflow GameflowName)))
    (:`Is Not Valid`
      (return false false))))

(fn `LoadGameflow`
  (params (GameflowName :type Name))
  (`/Game/LabyrinthCore/Blueprints/CoreSystem/BPFL_Common.RemoteEvent` null (`/Game/LabyrinthCore/Blueprints/Library/BPFL_Labyrinth.AppendName` GameflowName "_Begin")))

(fn `PlayGameflow`
  (params (GameflowName :type Name))
  (bind _gamestate (`/Game/LabyrinthCore/Blueprints/CoreSystem/BPFL_Common.GetGameStateBP` null))
  (`/Engine/EditorBlueprintResources/StandardMacros.IsValid` _gamestate
    (:`Is Valid`
      (`/Game/LabyrinthCore/Blueprints/BP_GameState.SetCurrentGameflow` _gamestate (`local.GameflowName`))
      (`/Game/LabyrinthCore/Blueprints/CoreSystem/BPFL_Common.RemoteEvent` null (`/Game/LabyrinthCore/Blueprints/Library/BPFL_Labyrinth.AppendName` (`local.GameflowName`) "_Play")))))

(fn `UnloadGameflow`
  (params (GmeflowName :type Name))
  (`/Game/LabyrinthCore/Blueprints/CoreSystem/BPFL_Common.RemoteEvent` null (`/Game/LabyrinthCore/Blueprints/Library/BPFL_Labyrinth.AppendName` GmeflowName "_End")))