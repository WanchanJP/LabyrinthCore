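; BP_Sequencer is a playback controller for level sequences, offering play, stop, pause toggle, fast-forward and rewind.
; Play stores the given sequence player, and the other playback events act on it after a validity check.
; Seeking jumps from the current time by a frame-delta-scaled skip amount that varies with whether the sequence is playing.
; It also stores a settable origin transform and returns it through GetActorTransform.
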(event `/Game/LabyrinthCore/Blueprints/CoreSystem/BPIF_Sequencer.Play`
  (params (SequencePlayer :type "LevelSequencePlayer Object Reference"))
  ;[0 0 1] 再生
  (`/Engine/EditorBlueprintResources/StandardMacros.IsValid` SequencePlayer
    (:`Is Valid`
      (bind _output_get (set `self.SequencerPlayer` SequencePlayer))
      (`MovieSceneSequencePlayer.Play` _output_get))))

(event `/Game/LabyrinthCore/Blueprints/CoreSystem/BPIF_Sequencer.SetActorTransform`
  (params (Transform :type "Transform Structure"))
  (set `self.TransformOrigin` Transform))

(event `/Game/LabyrinthCore/Blueprints/CoreSystem/BPIF_Sequencer.Stop`
  (bind _sequencerplayer (`self.SequencerPlayer`))
  ;[0 0 1] 停止
  (`/Engine/EditorBlueprintResources/StandardMacros.IsValid` _sequencerplayer
    (:`Is Valid`
      (`MovieSceneSequencePlayer.Stop` _sequencerplayer))))

(event `/Game/LabyrinthCore/Blueprints/CoreSystem/BPIF_Sequencer.Pause`
  (bind _sequencerplayer (`self.SequencerPlayer`))
  ;[0 0 1] 一時停止
  (`/Engine/EditorBlueprintResources/StandardMacros.IsValid` _sequencerplayer
    (:`Is Valid`
      (if (`MovieSceneSequencePlayer.IsPaused` _sequencerplayer)
        (`MovieSceneSequencePlayer.Play` _sequencerplayer)
        (else
          (`MovieSceneSequencePlayer.Pause` _sequencerplayer))))))

(event `/Game/LabyrinthCore/Blueprints/CoreSystem/BPIF_Sequencer.FastForward`
  (bind _sequencerplayer (`self.SequencerPlayer`))
  ;[0 0 1] 早送り
  (`/Engine/EditorBlueprintResources/StandardMacros.IsValid` _sequencerplayer
    (:`Is Valid`
      (`MovieSceneSequencePlayer.JumpToSeconds` _sequencerplayer (+ (`TimeManagementBlueprintLibrary.Conv_QualifiedFrameTimeToSeconds` (`MovieSceneSequencePlayer.GetCurrentTime` _sequencerplayer)) (* (`KismetMathLibrary.SelectFloat` (`self.SequencerSkipTime`) (+ (`self.SequencerSkipTime`) 1.0) (`MovieSceneSequencePlayer.IsPlaying` _sequencerplayer)) (`GameplayStatics.GetWorldDeltaSeconds`)))))))

(event `/Game/LabyrinthCore/Blueprints/CoreSystem/BPIF_Sequencer.Rewind`
  (bind _sequencerplayer (`self.SequencerPlayer`))
  ;[0 0 1] 巻き戻し
  (`/Engine/EditorBlueprintResources/StandardMacros.IsValid` _sequencerplayer
    (:`Is Valid`
      (`MovieSceneSequencePlayer.JumpToSeconds` _sequencerplayer (- (`TimeManagementBlueprintLibrary.Conv_QualifiedFrameTimeToSeconds` (`MovieSceneSequencePlayer.GetCurrentTime` _sequencerplayer)) (* (`KismetMathLibrary.SelectFloat` (+ (`self.SequencerSkipTime`) 2.0) (+ (`self.SequencerSkipTime`) 1.0) (`MovieSceneSequencePlayer.IsPlaying` _sequencerplayer)) (`GameplayStatics.GetWorldDeltaSeconds`)))))))

(fn `GetActorTransform`
  (returns (Transform :type "Transform Structure"))
  (return (`self.TransformOrigin`)))

(fn `UserConstructionScript`
  (`parent.UserConstructionScript`))