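; BP_DebugGameMode is a game mode Blueprint that adds a debug UI during play.
; On BeginPlay it creates the WB_DebugUI widget and adds it to the viewport at the debug Z-order, but only outside builds packaged for distribution.
; EndPlay removes the widget.
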(event `self.ReceiveBeginPlay`
  (`parent.ReceiveBeginPlay`)
  ;[1 1 1] Debug用UMG追加
  (if (not (`KismetSystemLibrary.IsPackagedForDistribution`))
    (`/Game/LabyrinthCore/Blueprints/Library/Actor/BPML_Widget.LbCreateWidget` "/Game/LabyrinthCore/Blueprints/Debug/WB_DebugUI.WB_DebugUI_C" (`self.WB_DebugUI`) true (`/Game/LabyrinthCore/Blueprints/Const/BPCST_WidgetPriority.WPr_Debug`))))

(event `self.ReceiveEndPlay`
  (params (EndPlayReason :type "EEndPlayReason Enum" :default "Destroyed"))
  (`parent.ReceiveEndPlay` EndPlayReason)
  (`/Game/LabyrinthCore/Blueprints/Library/Actor/BPML_Widget.LbRemoveWidget` (`self.WB_DebugUI`)))

(fn `UserConstructionScript`
  (`parent.UserConstructionScript`))