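; BP_Pickup is a pickup actor with a spring arm that can be turned relative to a given location, apparently for a zoom view.
; BeginPlay caches the arm's initial relative rotation.
; SetArmForwardPlayer combines it with the horizontal look-at rotation from that location to the actor and applies the result in world space.
; PickupBegin, noted as called on zoom, and PickupEnd are empty events.
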(event `self.ReceiveBeginPlay`
  ;[1 0 0] Begin
  (`parent.ReceiveBeginPlay`)
  (set `self.SpringArmInitialRotator` (`SceneComponent.RelativeRotation` (`self.SpringArm`))))

(event `PickupBegin`
  ;[1 1 1] Zoom時に呼ばれる
)

(event `PickupEnd`
  ;[1 1 1] Zoom時に呼ばれる
)

(fn `SetArmForwardPlayer`
  (params (Location :type "Vector Structure"))
  (bind (_returnvalue_x _returnvalue_y) (`KismetMathLibrary.BreakVector` (`self.K2_GetActorLocation`)))
  (`SceneComponent.K2_SetWorldRotation` (`self.SpringArm`) (`KismetMathLibrary.ComposeRotators` (`self.SpringArmInitialRotator`) (`KismetMathLibrary.FindLookAtRotation` (`KismetMathLibrary.MakeVector` (.x Location) (.y Location)) (`KismetMathLibrary.MakeVector` _returnvalue_x _returnvalue_y))) false false))

(fn `UserConstructionScript`)