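; Player component that runs the item pickup sequence as a camera cutscene, driving player states throughout.
; ExecutePickup stores the prior state, then blends the camera to the item while fading out the character.
; Once faded, it captures the scene as background, adds the item to inventory, and shows an off-map viewer copy with a dialog.
; PickupZoomOut reverses the blend and fade, restores the state, and destroys the item.
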(event `self.ReceiveBeginPlay`
  (bind _wb_pickupdialog (`self.WB_PickupDialog`))
  ;[1 0 0] Begin
  (`/Game/LabyrinthCore/Blueprints/Library/ActorComponent/BPML_Widget.LbCreateWidget` "/Game/LabyrinthCore/Blueprints/WidgetBP/WB_PickupDialog.WB_PickupDialog_C" _wb_pickupdialog true (`/Game/LabyrinthCore/Blueprints/Const/BPCST_WidgetPriority.WPr_PickupItem`))
  (`Widget.SetVisibility` _wb_pickupdialog "Hidden"))

(event `ExecutePickup`
  (params (PickupItem :type "/Game/LabyrinthCore/Blueprints/BP_Pickup Object Reference"))
  ;[1 0 0] アイテムを拾う処理を実行
  (`/Game/LabyrinthCore/Blueprints/Library/ActorComponent/BPML_PlayerState.LbIsPlayerState` (`/Game/LabyrinthCore/Blueprints/Const/BPCST_PlayerState.Pst_Ingame_LockPickup`)
    (:`false`
      (bind _playerstate (`/Game/LabyrinthCore/Blueprints/Library/ActorComponent/BPML_PlayerState.LbGetPlayerState`)
        (:`Succeeded`
          (set `self.PrevPlayerState` _playerstate) ; 拾い終わったら元のステートに戻るために保管しておく
          (set `self.PickupItem` PickupItem)
          (`self.ZoomIn`))))))

(event `ZoomIn`
  (bind _pickupitem (`self.PickupItem`))
  ;[0 0 1] ズームイン開始
  (`/Game/LabyrinthCore/Blueprints/Library/ActorComponent/BPML_PlayerState.LbSetPlayerState` (`/Game/LabyrinthCore/Blueprints/Const/BPCST_PlayerState.PSt_Pickup_ZoomIn`))
  (bind _playercharacter (`/Game/LabyrinthCore/Blueprints/Library/ActorComponent/BPML_Player.LbGetPlayerCharacter`)
    (:`Succeeded`
      (`/Game/LabyrinthCore/Blueprints/BP_Pickup.SetArmForwardPlayer` _pickupitem (`/Game/LabyrinthCore/Blueprints/BP_PlayerCharacter.GetCameraWorldLocation` _playercharacter)) ; Pickupアイテムのカメラアームをプレイヤーに向ける
      (`self.SetViewTarget` _pickupitem (`self.PickupZoomTime`)) ; Pickupアイテムのカメラに徐々に切り替える
      (`/Game/LabyrinthCore/Blueprints/BP_PlayerCharacter.OpacityOutRequest` _playercharacter) ; 主人公を徐々に透明にする
      (add `/Game/LabyrinthCore/Blueprints/BP_PlayerCharacter.OpacityOutFinished` _playercharacter (delegate `PickupZoomInFinished`)) ; 透明になったらイベント呼び出し
      ;[1 0.5029 0] OnZoomInBegin
      (`self.OnZoomInBegin`))))

(event `PickupZoomInFinished`
  (bind _returnvalue (`/Game/LabyrinthCore/Blueprints/Const/BPCST_PlayerState.PSt_Pickup_Dialog`))
  (bind _wb_pickupdialog (`self.WB_PickupDialog`))
  (bind _itemdata (`/Game/LabyrinthCore/Blueprints/BP_Pickup.ItemData` (`self.PickupItem`)))
  ;[0 0 1] ズームイン完了
  (bind _playercharacter (`/Game/LabyrinthCore/Blueprints/Library/ActorComponent/BPML_Player.LbGetPlayerCharacter`)
    (:`Succeeded`
      (remove `/Game/LabyrinthCore/Blueprints/BP_PlayerCharacter.OpacityOutFinished` _playercharacter (delegate `PickupZoomInFinished`))
      (`KismetSystemLibrary.Delay` (`self.PickupZoomFinishDelay`)) ; ズーム完了後にもう一瞬待つ
      (`/Game/LabyrinthCore/Blueprints/Library/ActorComponent/BPML_PlayerState.LbSetPlayerState` _returnvalue)
      (`/Game/LabyrinthCore/Blueprints/Library/ActorComponent/BPML_ActorComponent.LbCaptureSceneByPlayerState` (`BlueprintGameplayTagLibrary.MakeGameplayTagContainerFromTag` _returnvalue)) ; 背景用にズーム完了状態で画面キャプチャ
      (`/Game/LabyrinthCore/Blueprints/Library/ActorComponent/BPML_Player.LbSetPlayerOpacity` 1.0) ; SetPlayerStateでキャラ非表示になるのでOpacityは戻す
      (`/Game/LabyrinthCore/Blueprints/Library/ActorComponent/BPML_InventoryComponent.LbAddInventoryItem` _itemdata) ; アイテム追加
      (`self.CreateViewerItem` _itemdata) ; アイテムアクター生成
      (`self.SetViewTarget` (`self.ViewerItem`)) ; 表示用アイテムにカメラ切り替え
      ;[1 1 1] 獲得UMG表示
      (`Widget.SetVisibility` _wb_pickupdialog "Visible")
      (`/Game/LabyrinthCore/Blueprints/WidgetBP/WB_PickupDialog.PlayMessage` _wb_pickupdialog (`KismetStringLibrary.Conv_NameToString` (`/Game/LabyrinthCore/Blueprints/Types/BP_ItemData.Name` (`/Game/LabyrinthCore/Blueprints/BP_Pickup.ItemData` (`self.PickupItem`)))))
      ;[1 0 0] 開始
      (`/Game/LabyrinthCore/Blueprints/BP_Item.PlayPickup` (`self.ViewerItem`))
      ;[1 0.5029 0] OnZoomInEnd
      (`self.OnZoomInEnd`))))

(event `PickupZoomOut`
  ;[0 0 1] ズームアウト開始
  (`/Game/LabyrinthCore/Blueprints/Library/ActorComponent/BPML_PlayerState.LbSetPlayerState` (`/Game/LabyrinthCore/Blueprints/Const/BPCST_PlayerState.PSt_Pickup_ZoomOut`))
  (`Widget.SetVisibility` (`self.WB_PickupDialog`) "Hidden") ; 獲得UMG非表示
  (`self.SetViewTarget` (`self.PickupItem`)) ; ズームアウト開始するためにPickupItemにカメラ切り替え
  (`self.DestroyViewerItem`) ; カメラ切り替えたのでアクター消してよい
  (bind _playercharacter (`/Game/LabyrinthCore/Blueprints/Library/ActorComponent/BPML_Player.LbGetPlayerCharacter`)
    (:`Succeeded`
      (`self.SetViewTarget` _playercharacter (`self.PickupZoomTime`)) ; 主人公のカメラに徐々に切り替える
      (`/Game/LabyrinthCore/Blueprints/BP_PlayerCharacter.OpacityInRequest` _playercharacter) ; 主人公を徐々に不透明にする
      (add `/Game/LabyrinthCore/Blueprints/BP_PlayerCharacter.OpacityInFinished` _playercharacter (delegate `PickupZoomOutFinished`))
      (`Actor.SetActorHiddenInGame` (`self.PickupItem`) true) ; Pickupアイテムは入手したのでマップ上から非表示(まだDestroyしない)
      ;[1 0.5 0] OnZoomOutBegin
      (`self.OnZoomOutBegin`))))

(event `PickupZoomOutFinished`
  (bind _pickupitem (`self.PickupItem`))
  ;[0 0 1] ズームアウト完了
  (`/Game/LabyrinthCore/Blueprints/Library/ActorComponent/BPML_PlayerState.LbSetPlayerStateContainer` (`self.PrevPlayerState`))
  (`/Game/LabyrinthCore/Blueprints/BP_Pickup.PickupEnd` _pickupitem)
  (`Actor.K2_DestroyActor` _pickupitem)
  (set `self.PickupItem` null)
  ;[1 0.5 0] OnZoomOutEnd
  (`self.OnZoomOutEnd`))