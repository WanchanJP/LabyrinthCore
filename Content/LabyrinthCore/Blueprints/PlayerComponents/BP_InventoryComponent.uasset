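; Player inventory component for the Labyrinth game that holds collected items and drives the WB_InventorySystem widget it creates on BeginPlay.
; Adding or removing items by slot or tag rebuilds the widget's icons.
; Tapping a slot selects it and fires a selection-changed event; tapping it again begins or switches item analysis, gated by player-state gameplay tags.
; The back button ends analysis, and widget visibility is toggled externally.
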(event `self.ReceiveBeginPlay`
  ;[1 0 0] Begin
  (`/Game/LabyrinthCore/Blueprints/Library/ActorComponent/BPML_Widget.LbCreateWidget` "/Game/LabyrinthCore/Blueprints/WidgetBP/WB_InventorySystem.WB_InventorySystem_C" (`self.WB_Inventory`) true (`/Game/LabyrinthCore/Blueprints/Const/BPCST_WidgetPriority.WPr_Inventory`)))

(event `PushedItemButton`
  (params (SlotId :type Integer))
  (bind _wb_inventory (`self.WB_Inventory`))
  (bind _output (`|GetArrayItem` (`self.InventoryItems`) SlotId))
  ;[0 0 1] アイテムアイコンをタッチした
  (`self.IsSlotIdValid` SlotId
    (:`True`
      (if (== SlotId (`self.SelectedSlotId`))
        (`/Game/LabyrinthCore/Blueprints/Library/ActorComponent/BPML_PlayerState.LbIsPlayerState` (`/Game/LabyrinthCore/Blueprints/Const/BPCST_PlayerState.PSt_AnalyzeItem`) ; 既に調べ中かどうか
          (:`true`
            (`self.IsSameAnalyzeItem` (`/Game/LabyrinthCore/Blueprints/Types/BP_ItemData.ItemType` _output)
              (:`False`
                ;[1 1 0] 分析中のアイテムを変更する
                (`/Game/LabyrinthCore/Blueprints/Library/ActorComponent/BPML_AnalyzeItemComponent.LbChangeAnalyzeItem` _output))))
          (:`false`
            (`/Game/LabyrinthCore/Blueprints/Library/ActorComponent/BPML_PlayerState.LbIsPlayerState` (`/Game/LabyrinthCore/Blueprints/Const/BPCST_PlayerState.Pst_Ingame_LockAnalyze`)
              (:`false`
                (`/Game/LabyrinthCore/Blueprints/Library/ActorComponent/BPML_PlayerState.LbHasAnyPlayerState` (`BlueprintGameplayTagLibrary.MakeGameplayTagContainerFromArray` (`|MakeArray` (`/Game/LabyrinthCore/Blueprints/Const/BPCST_PlayerState.PSt_AnalyzeItem`) (`/Game/LabyrinthCore/Blueprints/Const/BPCST_PlayerState.PSt_Gimmick_Main`) (`/Game/LabyrinthCore/Blueprints/Const/BPCST_PlayerState.PSt_Ingame`)))
                  (:`true`
                    ;[1 1 0] 分析を開始する
                    (`/Game/LabyrinthCore/Blueprints/Library/ActorComponent/BPML_AnalyzeItemComponent.LbBeginAnalyzeItem` (`|GetArrayItem` (`self.InventoryItems`) SlotId))))))))
        (else
          (bind _output_get (set `self.SelectedSlotId` SlotId))
          (`/Engine/EditorBlueprintResources/StandardMacros.IsValid` _wb_inventory
            (:`Is Valid`
              (`/Game/LabyrinthCore/Blueprints/WidgetBP/WB_InventorySystem.ChangeSelectedItem` _wb_inventory _output_get)
              ;[1 1 0] 装備中のアイテムを変更する
              (`self.OnSelectedItemChanged` _output_get))))))))

(event `PushedBackButton`
  ;[0 0 1] 戻るボタンをタッチした
  ;[1 1 0.003] 分析を終了する
  (`/Game/LabyrinthCore/Blueprints/Library/ActorComponent/BPML_AnalyzeItemComponent.LbEndAnalyzeItem`))

(event `UpdateInventoryWidget`
  (bind _wb_inventory (`self.WB_Inventory`))
  ;[0 0 1] アイテムリストを更新する
  (`/Engine/EditorBlueprintResources/StandardMacros.IsValid` _wb_inventory
    (:`Is Valid`
      (`/Game/LabyrinthCore/Blueprints/WidgetBP/WB_InventorySystem.ClearAllItemTextures` _wb_inventory)
      (for (_array_element _array_index) (`self.InventoryItems`)
        (`/Game/LabyrinthCore/Blueprints/WidgetBP/WB_InventorySystem.SetItemTexture` _wb_inventory _array_index (`/Game/LabyrinthCore/Blueprints/Types/BP_ItemData.Icon` _array_element))))))

(fn `AddItem`
  (params (Item :type "/Game/LabyrinthCore/Blueprints/Types/BP_ItemData Object Reference"))
  (`/Engine/EditorBlueprintResources/StandardMacros.IsValid` Item
    (:`Is Valid`
      (`KismetArrayLibrary.Array_AddUnique` (`self.InventoryItems`) Item)
      (`self.UpdateInventoryWidget`))))

(fn `GetItem`
  (params (SlotId :type Integer))
  (returns (Item :type "/Game/LabyrinthCore/Blueprints/Types/BP_ItemData Object Reference"))
  (`self.IsSlotIdValid` SlotId
    (:`True`
      (return (`|GetArrayItem` (`self.InventoryItems`) SlotId)))))

(fn `SetVisibility`
  (params (bNewVisibility :type Boolean))
  (bind _wb_inventory (`self.WB_Inventory`))
  (`/Engine/EditorBlueprintResources/StandardMacros.IsValid` _wb_inventory
    (:`Is Valid`
      (if bNewVisibility
        (`Widget.SetVisibility` _wb_inventory "SelfHitTestInvisible")
        (else
          (`Widget.SetVisibility` _wb_inventory "Hidden"))))))

(fn `SubItemBySlotId`
  (params (SlotId :type Integer))
  (`KismetArrayLibrary.Array_Remove` (`self.InventoryItems`) SlotId)
  (`self.UpdateInventoryWidget`))

(fn `SubItemByTag`
  (params (ItemType :type "GameplayTag Structure"))
  (bind _inventoryitems (`self.InventoryItems`))
  (for (_array_element _array_index) _inventoryitems
    (if (== ItemType (`/Game/LabyrinthCore/Blueprints/Types/BP_ItemData.ItemType` _array_element))
      (`KismetArrayLibrary.Array_Remove` _inventoryitems _array_index)))
  (`self.UpdateInventoryWidget`))