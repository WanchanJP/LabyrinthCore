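; Player component that holds the player's current state as a gameplay tag container and applies it to the character.
; SetPlayerState replaces the tags, activates CharacterMovement only while an Ingame tag is present, and hides the player during CutScene.
; Query helpers offer exact, hierarchical and any-of tag matching.
; AddPlayerState only appends a tag, without refreshing movement or visibility.
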(fn `AddPlayerState`
  (params (Tag :type "GameplayTag Structure"))
  (`BlueprintGameplayTagLibrary.AddGameplayTag` (`self.PlayerState`) Tag))

(fn `GetPlayerState`
  (returns (PlayerState :type "GameplayTagContainer Structure"))
  (return (`self.PlayerState`)))

(fn `HasAnyPlayerState`
  (params (TagContainer :type "GameplayTagContainer Structure"))
  (returns (ReturnValue :type Boolean))
  (return (`BlueprintGameplayTagLibrary.HasAnyTags` (`self.PlayerState`) TagContainer)))

(fn `HasPlayerState`
  (params (Tag :type "GameplayTag Structure"))
  (returns (ReturnValue :type Boolean))
  (return (`BlueprintGameplayTagLibrary.HasTag` (`self.PlayerState`) Tag)))

(fn `IsPlayerState`
  (params (Tag :type "GameplayTag Structure"))
  (returns (ReturnValue :type Boolean))
  (return (`BlueprintGameplayTagLibrary.HasTag` (`self.PlayerState`) Tag true)))

(fn `SetPlayerState`
  (params (PlayerState :type "GameplayTagContainer Structure"))
  (set `self.PlayerState` PlayerState)
  (`|ExecutionSequence`
    (:`then_0`
      ;[1 1 1] CharacterMovement 有効/無効
      (if (`self.HasPlayerState` (struct :`TagName` "PlayerState.Ingame"))
        (bind _playercharacter (`/Game/LabyrinthCore/Blueprints/Library/ActorComponent/BPML_Player.LbGetPlayerCharacter`)
          (:`Succeeded`
            (`self.SetActive` (`Character.CharacterMovement` (stale _playercharacter_2)) true false)))
        (else
          (bind _playercharacter_2 (`/Game/LabyrinthCore/Blueprints/Library/ActorComponent/BPML_Player.LbGetPlayerCharacter`)
            (:`Succeeded`
              (`self.SetActive` false))))))
    (:`then_1`
      ;[1 1 1] キャラクターの表示/非表示
      (if (`self.HasAnyPlayerState` (struct :`GameplayTags` (struct :`(TagName` "PlayerState.CutScene") :`(TagName` "PlayerState.Gimmick.Cutscene") :`(TagName` "PlayerState.Gimmick.Main") :`(TagName` "PlayerState.Pickup.Dialog") :`(TagName` "PlayerState.Initialize"))))
        (`/Game/LabyrinthCore/Blueprints/Library/ActorComponent/BPML_Player.LbSetPlayerVisibility` false)
        (else
          (`/Game/LabyrinthCore/Blueprints/Library/ActorComponent/BPML_Player.LbSetPlayerVisibility` true))))))