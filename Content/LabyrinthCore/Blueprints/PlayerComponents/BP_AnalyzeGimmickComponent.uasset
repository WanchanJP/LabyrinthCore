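; Player component that runs the gimmick inspection mode, zooming the view into a gimmick and back to the character.
; ExecuteGimmick saves the player state, begins analysis, blends the camera to the gimmick and fades out the player.
; Opacity-finished callbacks advance player states, show the analyze widget on arrival, and on zoom-out end analysis and restore the saved state.
; Dispatchers report zoom phases and back-button presses.
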(event `self.ReceiveBeginPlay`
  (`/Game/LabyrinthCore/Blueprints/Library/ActorComponent/BPML_Widget.LbCreateWidget` "/Game/LabyrinthCore/Blueprints/WidgetBP/WB_Gimmick.WB_Gimmick_C" (`self.WB_AnalyzeGimmick`) true (`/Game/LabyrinthCore/Blueprints/Const/BPCST_WidgetPriority.WPr_AnalyzeGimmick`)))

(event `BeginAnalyzeGimmick`
  ;[1 1 1] 開始と終了
)

(event `EndAnalyzeGimmick`
  ;[1 1 1] 開始と終了
)

(event `SetBackButtonVisibility`
  (params (bNewVisibility :type Boolean))
  ;[1 1 1] 表示/非表示 切り替え
  (`/Game/LabyrinthCore/Blueprints/WidgetBP/WB_Gimmick.SetBackButtonVisibility` (`self.WB_AnalyzeGimmick`) bNewVisibility))

(event `ExecuteGimmick`
  (params (Gimmick :type "/Game/LabyrinthCore/Blueprints/BP_Gimmick Object Reference"))
  ;[1 0 0] ギミックを調べる処理を実行
  (bind _playerstate (`/Game/LabyrinthCore/Blueprints/Library/ActorComponent/BPML_PlayerState.LbGetPlayerState`)
    (:`Succeeded`
      (set `self.PrevPlayerState` _playerstate) ; 拾い終わったら元のステートに戻るために保管しておく
      (set `self.Gimmick` Gimmick)
      (`self.ZoomIn`))))

(event `PushedBackButton`
  ;[1 1 1] 戻るボタン
  (`self.OnPushedBackButton`))

(event `ZoomIn`
  ;[0 0 1] ズームイン開始
  (`/Game/LabyrinthCore/Blueprints/Library/ActorComponent/BPML_PlayerState.LbSetPlayerState` (`/Game/LabyrinthCore/Blueprints/Const/BPCST_PlayerState.PSt_Gimmick_ZoomIn`))
  ;[1 0 0] 開始
  (`/Game/LabyrinthCore/Blueprints/BP_Gimmick.BeginAnalyze` (`self.Gimmick`))
  (`self.SetViewTarget` (`self.Gimmick`)) ; ギミックのカメラに徐々に切り替える
  (bind _playercharacter (`/Game/LabyrinthCore/Blueprints/Library/ActorComponent/BPML_Player.LbGetPlayerCharacter`)
    (:`Succeeded`
      (`/Game/LabyrinthCore/Blueprints/Library/ActorComponent/BPML_Player.LbSetPlayerOpacityFadeOut`) ; 主人公を徐々に透明にする
      (add `/Game/LabyrinthCore/Blueprints/BP_PlayerCharacter.OpacityOutFinished` _playercharacter (delegate `ZoomInFinished`)) ; 透明になったらイベント呼び出し
      ;[1 0.5029 0] OnZoomInBegin
      (`self.OnZoomInBegin`))))

(event `ZoomInFinished`
  ;[0 0 1] ズームイン完了
  (bind _playercharacter (`/Game/LabyrinthCore/Blueprints/Library/ActorComponent/BPML_Player.LbGetPlayerCharacter`)
    (:`Succeeded`
      (remove `/Game/LabyrinthCore/Blueprints/BP_PlayerCharacter.OpacityOutFinished` _playercharacter (delegate `ZoomInFinished`))
      (`/Game/LabyrinthCore/Blueprints/Library/ActorComponent/BPML_PlayerState.LbSetPlayerState` (`/Game/LabyrinthCore/Blueprints/Const/BPCST_PlayerState.PSt_Gimmick_Main`))
      (`/Game/LabyrinthCore/Blueprints/Library/ActorComponent/BPML_Player.LbSetPlayerOpacity` 1.0) ; SetPlayerStateでキャラ非表示になるのでOpacityは戻す
      (`Widget.SetVisibility` (`self.WB_AnalyzeGimmick`) "Visible")
      ;[1 0.5 0] ZoomInEnd
      (`self.OnZoomInEnd`))))

(event `ZoomOut`
  ;[0 0 1] ズームアウト開始
  (`/Game/LabyrinthCore/Blueprints/Library/ActorComponent/BPML_PlayerState.LbSetPlayerState` (`/Game/LabyrinthCore/Blueprints/Const/BPCST_PlayerState.PSt_Gimmick_ZoomOut`))
  (`Widget.SetVisibility` (`self.WB_AnalyzeGimmick`) "Visible") ; 獲得UMG非表示
  (bind _playercharacter (`/Game/LabyrinthCore/Blueprints/Library/ActorComponent/BPML_Player.LbGetPlayerCharacter`)
    (:`Succeeded`
      (`self.SetViewTarget` _playercharacter) ; 主人公のカメラに徐々に切り替える
      (`/Game/LabyrinthCore/Blueprints/Library/ActorComponent/BPML_Player.LbSetPlayerOpacityFadeIn`)
      (add `/Game/LabyrinthCore/Blueprints/BP_PlayerCharacter.OpacityInFinished` _playercharacter (delegate `ZoomOutFinished`))
      ;[1 0.5 0] OnZoomOutBegin
      (`self.OnZoomOutBegin`))))

(event `ZoomOutFinished`
  ;[0 0 1] ズームアウト完了
  (bind _playercharacter (`/Game/LabyrinthCore/Blueprints/Library/ActorComponent/BPML_Player.LbGetPlayerCharacter`)
    (:`Succeeded`
      (remove `/Game/LabyrinthCore/Blueprints/BP_PlayerCharacter.OpacityInFinished` _playercharacter (delegate `ZoomOutFinished`))
      ;[1 0 0] 終了
      (`/Game/LabyrinthCore/Blueprints/BP_Gimmick.EndAnalyze` (`self.Gimmick`))
      (`/Game/LabyrinthCore/Blueprints/Library/ActorComponent/BPML_PlayerState.LbSetPlayerStateContainer` (`self.PrevPlayerState`))
      (set `self.Gimmick` null)
      ;[1 0.5 0] OnZoomOutEnd
      (`self.OnZoomOutEnd`))))