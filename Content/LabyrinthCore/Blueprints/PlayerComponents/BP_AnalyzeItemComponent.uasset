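; Player component that runs the item analysis (inspection) mode, showing an item up close with its own UI.
; Begin saves the player state, captures the scene as a background, spawns the item actor far from the origin and cuts the camera to it.
; Items can be swapped mid-analysis; ending restores the saved state and returns the view to the character or analyzed gimmick according to that state's tag.
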(event `self.ReceiveBeginPlay`
  ;[1 0 0] Begin
  (`/Game/LabyrinthCore/Blueprints/Library/ActorComponent/BPML_Widget.LbCreateWidget` "/Game/LabyrinthCore/Blueprints/WidgetBP/WB_AnalyzeItem.WB_AnalyzeItem_C" (`self.WB_Analyze`) true (`/Game/LabyrinthCore/Blueprints/Const/BPCST_WidgetPriority.WPr_AnalyzeItem`)))

(event `BeginAnalyze`
  (params (ItemData :type "/Game/LabyrinthCore/Blueprints/Types/BP_ItemData Object Reference"))
  ;[0 0 1] アイテム分析開始
  (bind _playerstate (`/Game/LabyrinthCore/Blueprints/Library/ActorComponent/BPML_PlayerState.LbGetPlayerState`)
    (:`Succeeded`
      (set `self.PrevPlayerState` _playerstate) ; 拾い終わったら元のステートに戻るために保管しておく
      (set `self.ItemData` ItemData)
      (`/Game/LabyrinthCore/Blueprints/Library/ActorComponent/BPML_PlayerState.LbSetPlayerState` (`/Game/LabyrinthCore/Blueprints/Const/BPCST_PlayerState.PSt_AnalyzeItem`))
      (`/Game/LabyrinthCore/Blueprints/Library/ActorComponent/BPML_ActorComponent.LbCaptureSceneByPlayerState` (`self.PrevPlayerState`)) ; 背景に表示するためのキャプチャ
      (`self.CreateAnalyzeItem` (`self.ItemData`)) ; アイテムアクター生成
      (`self.SetViewTarget` (`self.AnalyzingItem`)) ; 表示用アイテムにカメラ切り替え
      (`Widget.SetVisibility` (`self.WB_Analyze`) "Visible") ; UMG表示
      ;[1 0 0] 開始
      (`/Game/LabyrinthCore/Blueprints/BP_Item.BeginAnalyze` (`self.AnalyzingItem`))
      ;[1 0.5 0] OnBeginAnalyzeItem
      (`self.OnBeginAnalyzeItem`))))

(event `EndAnalyzeItem`
  (bind _prevplayerstate (`self.PrevPlayerState`))
  ;[0 0 1] アイテム分析終了
  (`/Game/LabyrinthCore/Blueprints/Library/ActorComponent/BPML_PlayerState.LbIsPlayerState` (`/Game/LabyrinthCore/Blueprints/Const/BPCST_PlayerState.PSt_AnalyzeItem`)
    (:`true`
      (`/Game/LabyrinthCore/Blueprints/Library/ActorComponent/BPML_PlayerState.LbSetPlayerStateContainer` _prevplayerstate)
      ;[1 1 1] プレイヤーステートによって戻り先のカメラが異なる
      (if (`BlueprintGameplayTagLibrary.HasTag` _prevplayerstate (`/Game/LabyrinthCore/Blueprints/Const/BPCST_PlayerState.PSt_Ingame`))
        (bind _playercharacter (`/Game/LabyrinthCore/Blueprints/Library/ActorComponent/BPML_Player.LbGetPlayerCharacter`)
          (:`Succeeded`
            (`self.SetViewTarget` _playercharacter)
            (`Widget.SetVisibility` (`self.WB_Analyze`) "Hidden" :!label _label) ; UMG非表示
            ;[1 0 0] 終了
            (`/Game/LabyrinthCore/Blueprints/BP_Item.EndAnalyze` (`self.AnalyzingItem`))
            (`self.DestroyAnalyzeItem`) ; アイテムアクター破棄
            ;[1 0.5 0] OnEndAnalyzeItem
            (`self.OnEndAnalyzeItem`)))
        (elif (`BlueprintGameplayTagLibrary.HasTag` _prevplayerstate (`/Game/LabyrinthCore/Blueprints/Const/BPCST_PlayerState.PSt_Gimmick`))
          (bind _analyzegimmickcomponent (`/Game/LabyrinthCore/Blueprints/Library/ActorComponent/BPML_GimmickComponent.LbGetAnalyzeGimmickComponent`)
            (:`Succeeded`
              (`self.SetViewTarget` (`/Game/LabyrinthCore/Blueprints/PlayerComponents/BP_AnalyzeGimmickComponent.Gimmick` _analyzegimmickcomponent))
              (goto _label)))
          (else
            (`KismetSystemLibrary.PrintString` "Error!")))))))

(event `ChangeAnalyzeItem`
  (params (ItemData :type "/Game/LabyrinthCore/Blueprints/Types/BP_ItemData Object Reference"))
  (bind _analyzingitem (`self.AnalyzingItem`))
  ;[0 0 1] 分析中にアイテム変更
  (`/Game/LabyrinthCore/Blueprints/Library/ActorComponent/BPML_PlayerState.LbIsPlayerState` (`/Game/LabyrinthCore/Blueprints/Const/BPCST_PlayerState.PSt_AnalyzeItem`)
    (:`true`
      ;[1 0 0] 終了
      (`/Game/LabyrinthCore/Blueprints/BP_Item.EndAnalyze` (`self.AnalyzingItem`))
      (`self.DestroyAnalyzeItem`)
      (bind _output_get (set `self.ItemData` ItemData))
      (`self.CreateAnalyzeItem` _output_get)
      (`self.SetViewTarget` _analyzingitem)
      ;[1 0 0] 開始
      (`/Game/LabyrinthCore/Blueprints/BP_Item.BeginAnalyze` _analyzingitem)
      ;[1 0.5 0] OnChangeAnalyzeItem
      (`self.OnChangeAnalyzeItem`))))

(fn `GetAnalyzingItem`
  (returns (AnalyzingItem :type "/Game/LabyrinthCore/Blueprints/BP_Item Object Reference"))
  (return (`self.AnalyzingItem`)))