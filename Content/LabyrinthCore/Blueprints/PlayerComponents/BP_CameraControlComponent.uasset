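; Player camera control component that turns touch gestures into inertial spring-arm orbit, FOV zoom and camera look rotation.
; Swipe, pinch and two-finger swipe add clamped speed while in-game and unlocked, with finger-delta dot product separating pinch from rotation on mobile.
; Tick applies FPS-adjusted speeds within limits and decays them.
; Zoom and look rotation ease back to default unless two fingers are down.
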(event Custom|OnSwipte
  (params (TouchIndex :type ETouchIndex%20Enum :default "Touch1"))
  (CallFunction|InputCameraMove))

(event Custom|OnPinch
  (CallFunction|InputCameraZoom))

(event Custom|OnTwoFingerSwipe
  (CallFunction|InputCameraRotation))

(event EventBeginPlay
  (Utilities|FlowControl|Sequence
    (:then_0
      (CallFunction|SetDefaultCameraParam))
    (:then_1
      (bind _playercontroller (Utilities|LbGetPlayerController)
        (:Succeeded
          (EventDispatchers|BindEventtoSwipe _playercontroller (delegate Custom|OnSwipte))
          (EventDispatchers|BindEventtoPinch _playercontroller (delegate Custom|OnPinch))
          (EventDispatchers|BindEventtoTwoFingerSwipe _playercontroller (delegate Custom|OnTwoFingerSwipe)))))))

(event Custom|InputCameraMove
  (bind _movemaxspeedy (Variables|Move|GetMoveMaxSpeedY))
  (bind _movemaxspeedx (Variables|Move|GetMoveMaxSpeedX))
  (Utilities|IsEnableCamera
    (:True
      (Utilities|FlowControl|Sequence
        (:then_0
          ;[1 1 1] 加速度の計算
          (bind _playercontroller (Utilities|LbGetPlayerController)
            (:Succeeded
              (Variables|Move|SetMoveAccelX (* (.x (Variables|/Game/LabyrinthCore/Blueprints/BP_PlayerController.BP_PlayerController_C|GetTouchDeltaLocation _playercontroller)) (Variables|Move|GetMoveAccelXRatio) 0.01))
              (Variables|Move|SetMoveAccelY (* (.y (Variables|/Game/LabyrinthCore/Blueprints/BP_PlayerController.BP_PlayerController_C|GetTouchDeltaLocation _playercontroller)) (Variables|Move|GetMoveAccelYRatio) 0.01)))))
        (:then_1
          ;[1 1 1] 算出した加速度をカメラ速度に反映
          (Variables|Move|SetMoveSpeedX (Math|Float|Clamp(Float) (+ (Variables|Move|GetMoveSpeedX) (Variables|Move|GetMoveAccelX)) (* _movemaxspeedx -1.0) _movemaxspeedx))
          (Variables|Move|SetMoveSpeedY (Math|Float|Clamp(Float) (+ (Variables|Move|GetMoveSpeedY) (Variables|Move|GetMoveAccelY)) (* _movemaxspeedy -1.0) _movemaxspeedy)))))))

(event Custom|InputCameraZoom
  (bind _zoommaxspeed (Variables|Zoom|GetZoomMaxSpeed))
  (Utilities|IsEnableCamera
    (:True
      (bind _playercontroller (Utilities|LbGetPlayerController)
        (:Succeeded
          (if (.bIsMobile (CallFunction|IsRunningonMobile)) ; True : モバイル実機
            (if (< (Variables|/Game/LabyrinthCore/Blueprints/BP_PlayerController.BP_PlayerController_C|GetTwoFingerDeltaDot _playercontroller) 0.0)
              (Utilities|FlowControl|Sequence :!label _label
                (:then_0
                  ;[1 1 1] 加速度の計算
                  (Variables|Zoom|SetZoomAccel (* (Variables|/Game/LabyrinthCore/Blueprints/BP_PlayerController.BP_PlayerController_C|GetTwoFingerDeltaLength _playercontroller) (Variables|Zoom|GetZoomAccelRatio) -0.01)))
                (:then_1
                  ;[1 1 1] 算出した加速度をズーム速度に反映
                  (Variables|Zoom|SetZoomSpeed (Math|Float|Clamp(Float) (+ (Variables|Zoom|GetZoomSpeed) (Variables|Zoom|GetZoomAccel)) (* _zoommaxspeed -1.0) _zoommaxspeed)))))
            (else
              ;[1 1 1] PCのときはマウスホイール操作なので指数０なら可
              (if (== (Variables|/Game/LabyrinthCore/Blueprints/BP_PlayerController.BP_PlayerController_C|GetFingerNum _playercontroller) 0)
                (goto _label)))))))))

(event Custom|InputCameraRotation
  (bind _rotatespeedymax (Variables|Rotation|GetRotateSpeedYMax))
  (bind _rotatespeedxmax (Variables|Rotation|GetRotateSpeedXMax))
  (Utilities|IsEnableCamera
    (:True
      (bind _playercontroller (Utilities|LbGetPlayerController)
        (:Succeeded
          (if (>= (Variables|/Game/LabyrinthCore/Blueprints/BP_PlayerController.BP_PlayerController_C|GetTwoFingerDeltaDot _playercontroller) 0.0)
            (Utilities|FlowControl|Sequence
              (:then_0
                ;[1 1 1] 加速度の計算
                (Variables|Rotation|SetRotateAccelX (* (.x (Variables|/Game/LabyrinthCore/Blueprints/BP_PlayerController.BP_PlayerController_C|GetTwoFingerTouchDeltaLocation _playercontroller)) (Variables|Rotation|GetRotateAccelRatio) 0.01))
                (Variables|Rotation|SetRotateAccelY (* (.y (Variables|/Game/LabyrinthCore/Blueprints/BP_PlayerController.BP_PlayerController_C|GetTwoFingerTouchDeltaLocation _playercontroller)) (Variables|Rotation|GetRotateAccelRatio) 0.01)))
              (:then_1
                ;[1 1 1] 算出した加速度をカメラ回転速度に反映
                (Variables|Rotation|SetRotateSpeedX (Math|Float|Clamp(Float) (+ (Variables|Rotation|GetRotateSpeedX) (Variables|Rotation|GetRotateAccelX)) (* _rotatespeedxmax -1.0) _rotatespeedxmax))
                (Variables|Rotation|SetRotateSpeedY (Math|Float|Clamp(Float) (+ (Variables|Rotation|GetRotateSpeedY) (Variables|Rotation|GetRotateAccelY)) (* _rotatespeedymax -1.0) _rotatespeedymax))))))))))

(event Custom|UpdateCameraMove
  (bind _defaultarmrotation (Variables|DefaultParameter|GetDefaultArmRotation))
  (Utilities|FlowControl|Sequence
    (:then_0
      ;[1 1 1] カメラ移動値を更新
      (Variables|Move|SetMoveX (|(((x+540)%360)-180) (+ (Variables|Move|GetMoveX) (CallFunction|ApplyValueatFPS (Variables|Move|GetMoveSpeedX)))))
      (Variables|Move|SetMoveY (Math|Float|Clamp(Float) (+ (Variables|Move|GetMoveY) (CallFunction|ApplyValueatFPS (Variables|Move|GetMoveSpeedY))) (Variables|Move|GetMoveYMin) (Variables|Move|GetMoveYMax))))
    (:then_1
      ;[1 1 1] カメラ位置を更新
      (bind _playercharacter (Utilities|LbGetPlayerCharacter)
        (:Succeeded
          (Transformation|SetWorldRotation (Variables|/Game/LabyrinthCore/Blueprints/BP_PlayerCharacter.BP_PlayerCharacter_C|GetSpringArm _playercharacter) (Math|Rotator|MakeRotator 0.0 (+ (.pitch _defaultarmrotation) (* (Variables|Move|GetMoveY) -1.0)) (+ (.yaw _defaultarmrotation) (Variables|Move|GetMoveX))) false false))))
    (:then_2
      ;[1 1 1] 速度を減衰させる
      (Variables|Move|SetMoveSpeedX (- (Variables|Move|GetMoveSpeedX) (CallFunction|ApplyValueatFPS (|(speed-(speed*decay)) (Variables|Move|GetMoveDecayX) (Variables|Move|GetMoveSpeedX)))))
      (Variables|Move|SetMoveSpeedY (- (Variables|Move|GetMoveSpeedY) (CallFunction|ApplyValueatFPS (|(speed-(speed*decay)) (Variables|Move|GetMoveDecayY) (Variables|Move|GetMoveSpeedY))))))))

(event Custom|UpdateCameraZoom
  (Utilities|FlowControl|Sequence
    (:then_0
      ;[1 1 1] ズーム値を更新
      (Variables|Zoom|SetZoom (Math|Float|Clamp(Float) (+ (Variables|Zoom|GetZoom) (CallFunction|ApplyValueatFPS (Variables|Zoom|GetZoomSpeed))) (Variables|Zoom|GetZoomMin) (Variables|Zoom|GetZoomMax))))
    (:then_1
      ;[1 1 1] ズーム反映
      (bind _playercharacter (Utilities|LbGetPlayerCharacter)
        (:Succeeded
          (Camera|SetFieldOfView (Variables|/Game/LabyrinthCore/Blueprints/BP_PlayerCharacter.BP_PlayerCharacter_C|GetCamera _playercharacter) (+ (Variables|DefaultParameter|GetDefaultFieldOfView) (* (Variables|Zoom|GetZoom) -1.0))))))
    (:then_2
      ;[1 1 1] ズーム速度を減衰させる
      (Variables|Zoom|SetZoomSpeed (* (Variables|Zoom|GetZoomSpeed) (Variables|Zoom|GetZoomSpeedDecay)))
      ;[1 1 1] 指を離すとズームを戻す
      (bind _playercontroller (Utilities|LbGetPlayerController)
        (:Succeeded
          (if (!= (Variables|/Game/LabyrinthCore/Blueprints/BP_PlayerController.BP_PlayerController_C|GetFingerNum _playercontroller) 2)
            (Variables|Zoom|SetZoom (* (Variables|Zoom|GetZoom) (Variables|Zoom|GetZoomDecay)))))))))

(event Custom|UpdateCameraRotation
  (bind _rotatedecay (Variables|Rotation|GetRotateDecay))
  (bind _rotatespeeddecay (Variables|Rotation|GetRotateSpeedDecay))
  (Utilities|FlowControl|Sequence
    (:then_0
      ;[1 1 1] Pan値を算出
      (Variables|Rotation|SetRotateX (Math|Float|Clamp(Float) (+ (Variables|Rotation|GetRotateX) (CallFunction|ApplyValueatFPS (Variables|Rotation|GetRotateSpeedX))) (Variables|Rotation|GetRotateXMin) (Variables|Rotation|GetRotateXMax)))
      (Variables|Rotation|SetRotateY (Math|Float|Clamp(Float) (+ (Variables|Rotation|GetRotateY) (CallFunction|ApplyValueatFPS (Variables|Rotation|GetRotateSpeedY))) (Variables|Rotation|GetRotateYMin) (Variables|Rotation|GetRotateYMax))))
    (:then_1
      ;[1 1 1] カメラ回転を反映
      (bind _playercharacter (Utilities|LbGetPlayerCharacter)
        (:Succeeded
          (Transformation|SetRelativeRotation (Variables|/Game/LabyrinthCore/Blueprints/BP_PlayerCharacter.BP_PlayerCharacter_C|GetCamera _playercharacter) (Math|Rotator|MakeRotator 0.0 (* (Variables|Rotation|GetRotateY) -1.0) (* (Variables|Rotation|GetRotateX) 1.0)) false false))))
    (:then_2
      ;[1 1 1] 回転速度を減衰させる
      (Variables|Rotation|SetRotateSpeedX (* (Variables|Rotation|GetRotateSpeedX) _rotatespeeddecay))
      (Variables|Rotation|SetRotateSpeedY (* (Variables|Rotation|GetRotateSpeedY) _rotatespeeddecay))
      ;[1 1 1] 指を離すと回転を戻す
      (bind _playercontroller (Utilities|LbGetPlayerController)
        (:Succeeded
          (if (!= (Variables|/Game/LabyrinthCore/Blueprints/BP_PlayerController.BP_PlayerController_C|GetFingerNum _playercontroller) 2)
            (Variables|Rotation|SetRotateX (* (Variables|Rotation|GetRotateX) _rotatedecay))
            (Variables|Rotation|SetRotateY (* (Variables|Rotation|GetRotateY) _rotatedecay))))))))

(event EventTick
  (params (DeltaSeconds :type Float%20%28single-precision%29))
  (CallFunction|UpdateCameraMove)
  (CallFunction|UpdateCameraZoom)
  (CallFunction|UpdateCameraRotation))

(fn SetDefaultCameraParam
  (bind _playercharacter (Utilities|LbGetPlayerCharacter)
    (:Succeeded
      (Variables|DefaultParameter|SetDefaultArmRotation (Transformation|GetActorRotation _playercharacter))
      (Variables|DefaultParameter|SetDefaultArmLocation (Variables|/Script/Engine.SceneComponent|GetRelativeLocation (Variables|/Game/LabyrinthCore/Blueprints/BP_PlayerCharacter.BP_PlayerCharacter_C|GetSpringArm _playercharacter)))
      (Variables|DefaultParameter|SetDefaultFieldOfView (Variables|/Script/Engine.CameraComponent|GetFieldOfView (Variables|/Game/LabyrinthCore/Blueprints/BP_PlayerCharacter.BP_PlayerCharacter_C|GetCamera _playercharacter))))))

(fn SetCameraMoveParam
  (params (MoveX :type Float%20%28single-precision%29) (MoveY :type Float%20%28single-precision%29))
  (Variables|Move|SetMoveX MoveX)
  (Variables|Move|SetMoveY MoveY))