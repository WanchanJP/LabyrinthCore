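; Player movement component that walks the player character along a synchronously found navigation path to a requested target location.
; Move requests store the path points and draw debug spheres at them.
; Tick replaces Move To, smoothly turning yaw toward the current point unless near, adding forward input for curved paths, and advancing points until the goal clears the path.
; CalcSpeed feeds MaxWalkSpeed, but its final-point slowdown calculation is unconnected.
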(event `self.ReceiveTick`
  (params (DeltaSeconds :type "Float (single-precision)"))
  (if (> (`KismetArrayLibrary.Array_Length` (`self.PathPoints`)) 0)
    (bind _playercharacter (`/Game/LabyrinthCore/Blueprints/Library/ActorComponent/BPML_Player.LbGetPlayerCharacter`)
      (:`Succeeded`
        (if (not (`self.IsAtLocation` (`self.GetCurrentPathPoint` _playercharacter) (`self.AcceptanceDist`) _playercharacter))
          ;[1 1 1] カスタムVerのMove To
          (if (not (`self.IsNear`))
            (bind (_returnvalue_roll _returnvalue_pitch _returnvalue_yaw) (`KismetMathLibrary.BreakRotator` (`KismetMathLibrary.RInterpTo` (`Actor.K2_GetActorRotation` _playercharacter) (`KismetMathLibrary.FindLookAtRotation` (`Actor.K2_GetActorLocation` _playercharacter) (`self.GetCurrentPathPoint` _playercharacter)) DeltaSeconds 2.0)))
            (`Actor.K2_SetActorRotation` _playercharacter (`KismetMathLibrary.MakeRotator` 0.0 0.0 _returnvalue_yaw) false))
          (set `CharacterMovementComponent.MaxWalkSpeed` (`KismetMathLibrary.SelectFloat` (* (- (`self.Dist`) (- (`self.AcceptanceDist`) 2.0)) (/ (`self.SpeedMax`) (- (`self.SpeedDownDist`) (`self.AcceptanceDist`)))) (`self.SpeedMax`) (and (`self.IsNear`) (== (- (`KismetArrayLibrary.Array_Length` (`self.PathPoints`)) 1) (`self.PointsIndex`)))) (`Character.CharacterMovement` _playercharacter))
          (`Pawn.AddMovementInput` _playercharacter (`Actor.GetActorForwardVector` _playercharacter) 1.0 false) ; 実際の移動はPawnの前方へAddMovementするだけ
          (else
            ;[0 0 0] インデックスの更新と最終目的地到達のチェック
            (bind _reacheddestination (`self.UpdatePathPointIndex`))
            (if _reacheddestination
              ;[0 0 0] 最終目的地に到達した後の処理
              (`KismetSystemLibrary.PrintString` "Goal Reached")
              (`KismetArrayLibrary.Array_Clear` (`self.PathPoints`)))))))))

(event `PlayerStartMoveRequest`
  (params (TargetLocation :type "Vector Structure"))
  (bind _playercharacter (`/Game/LabyrinthCore/Blueprints/Library/ActorComponent/BPML_Player.LbGetPlayerCharacter`)
    (:`Succeeded`
      ;[1 1 1] 目的地までの経路を探索し、結果を保持する
      (bind _returnvalue (`NavigationSystemV1.FindPathToLocationSynchronously` (`Actor.K2_GetActorLocation` _playercharacter) TargetLocation null null))
      (set `self.PathPoints` (`NavigationPath.PathPoints` _returnvalue))
      (set `self.PointsIndex` 0)
      (bind _playercharacter_2 (`/Game/LabyrinthCore/Blueprints/Library/ActorComponent/BPML_Player.LbGetPlayerCharacter`)
        (:`Succeeded`
          ;[1 0 0] DEBUG
          (for _array_element (`self.PathPoints`)
            (bind (_returnvalue_x _returnvalue_y _returnvalue_z) (`KismetMathLibrary.BreakVector` (`Actor.K2_GetActorLocation` _playercharacter_2)))
            (`KismetSystemLibrary.DrawDebugSphere` (`KismetMathLibrary.MakeVector` (.x _array_element) (.y _array_element) _returnvalue_z) 25.0 4 (struct :`R` 1.0 :`G` 1.0 :`A` 1.0) 5.0 2.0)))))))

(fn `GetCurrentPathPoint`
  (params (Target :type "Actor Object Reference"))
  (returns (Point :type "Vector Structure"))
  (bind (_returnvalue_x _returnvalue_y _returnvalue_z) (`KismetMathLibrary.BreakVector` (`Actor.K2_GetActorLocation` Target)))
  (bind _pathpoints (`self.PathPoints`))
  (bind _pointsindex (`self.PointsIndex`))
  (bind (_output_x _output_y) (`KismetMathLibrary.BreakVector` (`|GetArrayItem` _pathpoints _pointsindex)))
  (if (> _pointsindex (- (`KismetArrayLibrary.Array_Length` _pathpoints) 1))
    (`KismetSystemLibrary.PrintString` "ERROR : Out of Bounds" true true (struct :`R` 1.0 :`A` 1.0))
    (return (0.0 0.0 0.0))
    (else
      (return (`KismetMathLibrary.MakeVector` _output_x _output_y _returnvalue_z)))))

(fn `IsAtLocation`
  (params (Location :type "Vector Structure") (`Acceptance Dist` :type "Float (double-precision)" :default 5.0) (Target :type "Actor Object Reference"))
  (returns (ReturnValue :type Boolean))
  (bind _returnvalue (- Location (`Actor.K2_GetActorLocation` Target)))
  (set `self.Dist` (`KismetMathLibrary.VSize` _returnvalue))
  (return (<= (`KismetMathLibrary.VSizeSquared` _returnvalue) (`KismetMathLibrary.Square` `Acceptance Dist`))))

(fn `IsNear`
  (returns (ReturnValue :type Boolean))
  (return (< (`self.Dist`) (`self.SpeedDownDist`))))

(fn `UpdatePathPointIndex`
  (returns (ReachedDestination :type Boolean))
  (if (< (`self.PointsIndex`) (- (`KismetArrayLibrary.Array_Length` (`self.PathPoints`)) 1))
    (`/Engine/EditorBlueprintResources/StandardMacros.IncrementInt` (`self.PointsIndex`)
      (:`  `
        (return false)))
    (else
      (return true))))