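; BP_Gimmick is a labyrinth gimmick actor with analyze begin/end, overridable-looking empty state hooks, back-button exit and an inspection camera.
; Two-finger swipes and pinch (mouse wheel on PC) add acceleration to clamped move and zoom speeds.
; While camera control is enabled, Tick integrates and decays these speeds, then moves or rotates the camera target per axis and adjusts FOV.
; Camera parameters captured at BeginPlay are restored when analysis begins.
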(event `self.ReceiveTick`
  (params (DeltaSeconds :type "Float (single-precision)"))
  ;[1 0 0] Tick
  (`self.UpdateCameraControl`))

(event `self.ReceiveBeginPlay`
  ;[1 0 0] Begin
  (`self.SetDefaultCameraControlParam`))

(event `BeginState`
  ;[1 1 1] ステート管理系
)

(event `BeginAnalyze`
  ;[1 1 1] 開始時終了時に呼ばれるイベント
  (set `self.bAnalyzing` true)
  (`self.SetCameraControlParam` (`self.DefaultCameraParam`)))

(event `EndState`
  ;[1 1 1] ステート管理系
)

(event `EndAnalyze`
  ;[1 1 1] 開始時終了時に呼ばれるイベント
  (set `self.bAnalyzing` false))

(event `ChangeState`
  (params (NewGimmickState :type "GameplayTag Structure"))
  ;[1 1 1] ステート管理系
  (`self.EndState`)
  (set `self.GimmickState` NewGimmickState)
  (`self.BeginState`))

(event `CameraControlEnable`
  ;[1 1 1] Bind & Unbind
  (bind _playercontroller (`/Game/LabyrinthCore/Blueprints/Library/Actor/BPML_Player.LbGetPlayerController`)
    (:`Succeeded`
      (`self.SetActorTickEnabled` true)
      (add `/Game/LabyrinthCore/Blueprints/BP_PlayerController.TwoFingerSwipe` _playercontroller (delegate `EventMoveTwoFinger`))
      (add `/Game/LabyrinthCore/Blueprints/BP_PlayerController.Pinch` _playercontroller (delegate `EventPinch`))
      (set `self.bCameraControlEnable` true))))

(event `BackButtonExec`
  ;[1 1 1] 戻るボタン
  (`/Game/LabyrinthCore/Blueprints/Library/Actor/BPML_PlayerState.LbHasPlayerState` (`/Game/LabyrinthCore/Blueprints/Const/BPCST_PlayerState.PSt_Gimmick_Main`)
    (:`true`
      (`/Game/LabyrinthCore/Blueprints/Library/Actor/BPML_GimmickComponent.LbSetAnalyzeEnd`))))

(event `CameraControlDisable`
  ;[1 1 1] Bind & Unbind
  (bind _playercontroller (`/Game/LabyrinthCore/Blueprints/Library/Actor/BPML_Player.LbGetPlayerController`)
    (:`Succeeded`
      (`self.SetActorTickEnabled` false)
      (add `/Game/LabyrinthCore/Blueprints/BP_PlayerController.TwoFingerSwipe` _playercontroller (delegate `EventMoveTwoFinger`))
      (remove `/Game/LabyrinthCore/Blueprints/BP_PlayerController.Pinch` _playercontroller (delegate `EventPinch`))
      (set `self.bCameraControlEnable` false))))

(event `BackButtonEnable`
  ;[1 1 1] 戻るボタン
  (`/Game/LabyrinthCore/Blueprints/Library/Actor/BPML_GimmickComponent.LbSetBackButtonVisivility` true)
  (bind _analyzegimmickcomponent (`/Game/LabyrinthCore/Blueprints/Library/Actor/BPML_GimmickComponent.LbGetAnalyzeGimmickComponent`)
    (:`Succeeded`
      (add `/Game/LabyrinthCore/Blueprints/PlayerComponents/BP_AnalyzeGimmickComponent.OnPushedBackButton` _analyzegimmickcomponent (delegate `BackButtonExec`)))))

(event `EventMoveTwoFinger`
  ;[1 1 1] Bind & Unbind
  (`self.CalcMoveSpeed`))

(event `EventPinch`
  ;[1 1 1] Bind & Unbind
  (`self.CalcZoomSpeed`))

(event `BackButtonDisable`
  ;[1 1 1] 戻るボタン
  (`/Game/LabyrinthCore/Blueprints/Library/Actor/BPML_GimmickComponent.LbSetBackButtonVisivility` false)
  (bind _analyzegimmickcomponent (`/Game/LabyrinthCore/Blueprints/Library/Actor/BPML_GimmickComponent.LbGetAnalyzeGimmickComponent`)
    (:`Succeeded`
      (remove `/Game/LabyrinthCore/Blueprints/PlayerComponents/BP_AnalyzeGimmickComponent.OnPushedBackButton` _analyzegimmickcomponent (delegate `BackButtonExec`)))))

(event `CalcMoveSpeed`
  (bind (_defaulttargetlocation _defaulttargetrotation _defaultzoom _defaultspringarmlength _zoommin _zoommax _movemin _movemax _zoomaccel _zoomspeedmax _zoomdecay _moveaccel _movespeedmax) (break `/Game/LabyrinthCore/Blueprints/Types/FGimmickCameraParam` (`self.CurrentCameraParam`)))
  ;[1 1 1] MoveSpeed
  (bind _playercontroller (`/Game/LabyrinthCore/Blueprints/Library/Actor/BPML_Player.LbGetPlayerController`)
    (:`Succeeded`
      (bind (_twofingertouchdeltalocation_x _twofingertouchdeltalocation_y) (`KismetMathLibrary.BreakVector` (`/Game/LabyrinthCore/Blueprints/BP_PlayerController.TwoFingerTouchDeltaLocation` _playercontroller)))
      (bind _output_get (set `self.CameraMoveAccel` (`KismetMathLibrary.MakeVector2D` (* _twofingertouchdeltalocation_x _moveaccel 0.01) (* _twofingertouchdeltalocation_y _moveaccel 0.01 -1.0))))
      (set `self.CameraMoveSpeed` (`KismetMathLibrary.ClampAxes2D` (+ (`self.CameraMoveSpeed`) _output_get) (* _movespeedmax -1.0) _movespeedmax)))))

(event `UpdateCameraControl`
  (bind _cameratarget (`self.CameraTarget`))
  (bind _cameratarget_2 (`self.CameraTarget`))
  (bind _cameratarget_3 (`self.CameraTarget`))
  (bind _cameratarget_4 (`self.CameraTarget`))
  (bind (_defaulttargetlocation _defaulttargetrotation _defaultzoom _defaultspringarmlength _zoommin _zoommax _movemin _movemax) (break `/Game/LabyrinthCore/Blueprints/Types/FGimmickCameraParam` (`self.CurrentCameraParam`)))
  (bind (_defaulttargetlocation_2 _defaulttargetrotation_2 _defaultzoom_2 _defaultspringarmlength_2 _zoommin_2 _zoommax_2) (break `/Game/LabyrinthCore/Blueprints/Types/FGimmickCameraParam` (`self.CurrentCameraParam`)))
  (bind (_defaulttargetlocation_3 _defaulttargetrotation_3 _defaultzoom_3 _defaultspringarmlength_3 _zoommin_3 _zoommax_3 _movemin_2 _movemax_2 _zoomaccel _zoomspeedmax _zoomdecay _moveaccel _movespeedmax _movedecay _cameracontroltypex) (break `/Game/LabyrinthCore/Blueprints/Types/FGimmickCameraParam` (`self.CurrentCameraParam`)))
  (bind (_defaulttargetlocation_4 _defaulttargetrotation_4 _defaultzoom_4 _defaultspringarmlength_4 _zoommin_4 _zoommax_4 _movemin_3 _movemax_3 _zoomaccel_2 _zoomspeedmax_2 _zoomdecay_2 _moveaccel_2 _movespeedmax_2 _movedecay_2 _cameracontroltypex_2 _cameracontroltypey) (break `/Game/LabyrinthCore/Blueprints/Types/FGimmickCameraParam` (`self.CurrentCameraParam`)))
  (bind (_x _y) (`KismetMathLibrary.BreakVector2D` (`self.CameraMoveSpeed`)))
  (bind (_x_2 _y_2) (`KismetMathLibrary.BreakVector2D` (`self.CameraMove`)))
  (bind (_x_3 _y_3) (`KismetMathLibrary.BreakVector2D` (`self.CameraMove`)))
  (bind (_x_4 _y_4) (`KismetMathLibrary.BreakVector2D` (`self.CameraMove`)))
  (bind (_x_5 _y_5) (`KismetMathLibrary.BreakVector2D` _movemin))
  (bind (_x_6 _y_6) (`KismetMathLibrary.BreakVector2D` _movemax))
  ;[0 0 1] 速度を反映
  (`|ExecutionSequence`
    (:`then_0`
      ;[1 1 1] カメラ速度をカメラ回転値に反映
      (set `self.CameraMove` (`KismetMathLibrary.MakeVector2D` (`KismetMathLibrary.FClamp` (+ _x_2 (`/Game/LabyrinthCore/Blueprints/Library/BPFL_Labyrinth.ApplyValueAtFPS` _x)) _x_5 _x_6) (`KismetMathLibrary.FClamp` (+ _y_2 (`/Game/LabyrinthCore/Blueprints/Library/BPFL_Labyrinth.ApplyValueAtFPS` _y)) _y_5 _y_6)))
      ;[1 1 1] ズーム速度をズーム値に反映
      (set `self.CameraZoom` (`KismetMathLibrary.FClamp` (+ (`self.CameraZoom`) (`self.CameraZoomSpeed`)) _zoommin_2 _zoommax_2)))
    (:`then_1`
      ;[1 1 1] カメラ速度の減衰
      (set `self.CameraMoveSpeed` (* (`self.CameraMoveSpeed`) (`.MoveDecay_33_13CC26404A35190C65F6AAB3611BA4A7` (break `/Game/LabyrinthCore/Blueprints/Types/FGimmickCameraParam` (`self.CurrentCameraParam`)))))
      ;[1 1 1] ズーム速度の減衰
      (set `self.CameraZoomSpeed` (* (`self.CameraZoomSpeed`) (`.ZoomDecay_27_4EE5FFEF4268EF241CC64488F197D676` (break `/Game/LabyrinthCore/Blueprints/Types/FGimmickCameraParam` (`self.CurrentCameraParam`))))))
    (:`then_2`
      ;[1 1 1] カメラ操作の反映
      (if (`self.bCameraControlEnable`)
        (`|ExecutionSequence`
          (:`then_0`
            (switch `/Game/LabyrinthCore/Blueprints/Types/EGimmickCameraControlType` _cameracontroltypex
              (:`NewEnumerator1`
                (`SceneComponent.K2_SetRelativeLocation` _cameratarget_4 (`KismetMathLibrary.MakeVector` (.x (`SceneComponent.RelativeLocation` _cameratarget_2)) (.y (`SceneComponent.RelativeLocation` _cameratarget_2)) (+ (.z _defaulttargetlocation_3) _y_3)) false false))
              (:`NewEnumerator0`
                (`SceneComponent.K2_SetRelativeRotation` _cameratarget_4 (`KismetMathLibrary.MakeRotator` (.roll (`SceneComponent.RelativeRotation` _cameratarget_2)) (.pitch (`SceneComponent.RelativeRotation` _cameratarget_2)) (+ (.yaw _defaulttargetrotation_3) _x_3)) false false))))
          (:`then_1`
            (switch `/Game/LabyrinthCore/Blueprints/Types/EGimmickCameraControlType` _cameracontroltypey
              (:`NewEnumerator1`
                (`SceneComponent.K2_SetRelativeLocation` _cameratarget_3 (`KismetMathLibrary.MakeVector` (.x (`SceneComponent.RelativeLocation` _cameratarget)) (+ (.y _defaulttargetlocation_4) _x_4) (.z (`SceneComponent.RelativeLocation` _cameratarget))) false false))
              (:`NewEnumerator0`
                (`SceneComponent.K2_SetRelativeRotation` _cameratarget_3 (`KismetMathLibrary.MakeRotator` (.roll (`SceneComponent.RelativeRotation` _cameratarget)) (+ (.pitch _defaulttargetrotation_4) _y_4) (.yaw (`SceneComponent.RelativeRotation` _cameratarget))) false false))))
          (:`then_2`
            (`CameraComponent.SetFieldOfView` (`self.Camera`) (+ (`.DefaultZoom_8_B2E7994749E3A37579311EAD001A44BB` (break `/Game/LabyrinthCore/Blueprints/Types/FGimmickCameraParam` (`self.CurrentCameraParam`))) (* (`self.CameraZoom`) -1.0)))))))))

(event `CalcZoomSpeed`
  (bind (_defaulttargetlocation _defaulttargetrotation _defaultzoom _defaultspringarmlength _zoommin _zoommax _movemin _movemax _zoomaccel _zoomspeedmax) (break `/Game/LabyrinthCore/Blueprints/Types/FGimmickCameraParam` (`self.CurrentCameraParam`)))
  ;[1 1 1] ZoomSpeed
  (bind _playercontroller (`/Game/LabyrinthCore/Blueprints/Library/Actor/BPML_Player.LbGetPlayerController`)
    (:`Succeeded`
      (if (`/Game/LabyrinthCore/Blueprints/Library/BPFL_Labyrinth.IsRunningOnMobile`)
        (if (< (`/Game/LabyrinthCore/Blueprints/BP_PlayerController.TwoFingerDeltaDot` _playercontroller) 0.0)
          (bind _output_get (set `self.CameraZoomAccel` (* (`/Game/LabyrinthCore/Blueprints/BP_PlayerController.TwoFingerDeltaLength` _playercontroller) _zoomaccel -0.01) :!label _label))
          (set `self.CameraZoomSpeed` (`KismetMathLibrary.FClamp` (+ (`self.CameraZoomSpeed`) _output_get) (* _zoomspeedmax -1.0) _zoomspeedmax)))
        (else
          ;;[1 1 1] PCのときはマウスホイール操作なので指数０なら可
          (if (== (`/Game/LabyrinthCore/Blueprints/BP_PlayerController.FingerNum` _playercontroller) 0)
            (goto _label)))))))

(event `SetDefaultCameraControlParam`
  (bind _cameratarget (`self.CameraTarget`))
  ;[1 1 1] 初期状態の保存
  (set `self.DefaultCameraParam` (make `/Game/LabyrinthCore/Blueprints/Types/FGimmickCameraParam` (`SceneComponent.RelativeLocation` _cameratarget) (`SceneComponent.RelativeRotation` _cameratarget) (`CameraComponent.FieldOfView` (`self.Camera`)) (`SpringArmComponent.TargetArmLength` (`self.SpringArm`)))))

(event `SetCameraControlParam`
  (params (CameraControlParam :type "/Game/LabyrinthCore/Blueprints/Types/FGimmickCameraParam Structure"))
  (bind _cameratarget (`self.CameraTarget`))
  ;[1 1 1] カメラパラメータのセット
  (`|ExecutionSequence`
    (:`then_0`
      (bind _output_get (set `self.CurrentCameraParam` CameraControlParam))
      (bind (_defaulttargetlocation _defaulttargetrotation _defaultzoom _defaultspringarmlength) (break `/Game/LabyrinthCore/Blueprints/Types/FGimmickCameraParam` _output_get))
      (`SceneComponent.K2_SetRelativeLocation` _cameratarget _defaulttargetlocation false false)
      (`SceneComponent.K2_SetRelativeRotation` _cameratarget _defaulttargetrotation false false)
      (bind _output_get_2 (set `CameraComponent.FieldOfView` _defaultzoom (`self.Camera`)))
      (set `SceneCaptureComponent2D.FOVAngle` _output_get_2 (`self.SceneCaptureComponent2D`))
      (set `SpringArmComponent.TargetArmLength` _defaultspringarmlength (`self.SpringArm`)))
    (:`then_1`
      (set `self.CameraMove` (0.0 0.0))
      (set `self.CameraMoveAccel` (0.0 0.0))
      (set `self.CameraMoveSpeed` (0.0 0.0))
      (set `self.CameraZoom` 0.0))))

(fn `UserConstructionScript`)