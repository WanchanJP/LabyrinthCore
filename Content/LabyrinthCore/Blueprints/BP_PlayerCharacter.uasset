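; BP_PlayerCharacter is the Labyrinth player character, able to fade itself out and back in on request.
; OpacityOutRequest and OpacityInRequest play timelines that feed SetOpacity, then snap to the end value and fire a finished dispatcher.
; SetOpacity writes the HarukaOpacity scalar in the MPC_Labyrinth material parameter collection rather than touching materials directly.
; It also exposes the camera's world location through a getter.
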(event `self.ReceiveBeginPlay`
  (`KismetSystemLibrary.PrintString` "PlayerCharacter: BeginPlay" true true (struct :`G` 0.66 :`B` 1.0 :`A` 1.0) 4.0))

(event `OpacityOutRequest`
  ;[1 1 1] 徐々に透明にする
  (bind (_direction _opacity) (`Timeline|OpacityOut` :!via `PlayFromStart`)
    (:`Update`
      (`self.SetOpacity` _opacity))
    (:`Finished`
      (`self.SetOpacity` 0.0)
      (`self.OpacityOutFinished`))))

(event `OpacityInRequest`
  ;[1 1 1] 徐々に不透明にする
  (bind (_direction _opacity) (`Timeline|OpacityIn` :!via `PlayFromStart`)
    (:`Update`
      (`self.SetOpacity` _opacity))
    (:`Finished`
      (`self.SetOpacity` 1.0)
      (`self.OpacityInFinished`))))

(fn `GetCameraWorldLocation`
  (returns (Location :type "Vector Structure"))
  (return (`SceneComponent.K2_GetComponentLocation` (`self.Camera`))))

(fn `SetOpacity`
  (params (Opacity :type "Float (double-precision)"))
  (`KismetMaterialLibrary.SetScalarParameterValue` "/Game/LabyrinthCore/MaterialUtil/MPC_Labyrinth.MPC_Labyrinth" "HarukaOpacity" Opacity))

(fn `UserConstructionScript`)