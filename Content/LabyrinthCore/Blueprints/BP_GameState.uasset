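; Game state Blueprint that tracks the current and loaded gameflows as integer IDs.
; A settable gameflow data table drives conversion both ways: a row name yields its Value, and a Value search returns the row's Label.
; Setters store -1 when a name fails to resolve, while getters still report success and return None for unresolved IDs.
; It also lists the table's row names and compares a given gameflow against the current one.
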(event `SetGameflowDataTable`
  (params (GameflowDataTable :type "DataTable Object Reference"))
  (set `self.GameflowDataTable` GameflowDataTable))

(event `SetCurrentGameflow`
  (params (GameflowName :type Name))
  (bind _returnvalue (`self.ConvertNameToInt` GameflowName)
    (:`Succeeded`
      (set `self.CurrentGameflowID` _returnvalue))
    (:`Failed`
      (set `self.CurrentGameflowID` -1))))

(event `SetLoadedGameflow`
  (params (GameflowName :type Name))
  (bind _returnvalue (`self.ConvertNameToInt` GameflowName)
    (:`Succeeded`
      (set `self.LoadedGameflowID` _returnvalue))
    (:`Failed`
      (set `self.LoadedGameflowID` -1))))

(fn `GetCurrentGameflow`
  (returns (bSucceeded :type Boolean) (CurrentGameflow :type Name))
  (bind _returnvalue (`self.ConvertIntToName` (`self.CurrentGameflowID`))
    (:`Succeeded`
      (return true _returnvalue))
    (:`Failed`
      (return true "None"))))

(fn `GetGameflowList`
  (returns (bSucceeded :type Boolean) (GameflowList :type "Array of Name"))
  (bind _gameflowdatatable (`self.GameflowDataTable`))
  (`/Engine/EditorBlueprintResources/StandardMacros.IsValid` _gameflowdatatable
    (:`Is Valid`
      (bind _outrownames (`DataTableFunctionLibrary.GetDataTableRowNames` _gameflowdatatable))
      (return true _outrownames))
    (:`Is Not Valid`
      (return false))))

(fn `GetLoadedGameflow`
  (returns (bSucceeded :type Boolean) (LoadedGameflow :type Name))
  (bind _returnvalue (`self.ConvertIntToName` (`self.LoadedGameflowID`))
    (:`Succeeded`
      (return true _returnvalue))
    (:`Failed`
      (return true "None"))))

(fn `IsCurrentGameflow`
  (params (Gameflow :type Name))
  (returns (ReturnValue :type Boolean))
  (bind _returnvalue (`self.ConvertIntToName` (`self.CurrentGameflowID`))
    (:`Succeeded`
      (return (== Gameflow _returnvalue)))))

(fn `UserConstructionScript`)