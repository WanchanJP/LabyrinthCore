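; Player controller that turns touch input into gestures and handles tap-to-interact and tap-to-move.
; OnPress, OnMove and OnRelease track per-finger state and fire one- and two-finger press, release, swipe, tap and pinch events.
; Off mobile, mouse buttons emulate two fingers and the wheel drives pinch, with positions DPI-scaled like touch.
; In-game taps line-trace into the world to execute a BP_Pickup or BP_Gimmick, otherwise request movement unless locked.
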(event `self.ReceiveBeginPlay`
  ;[1 0 0] Begin
  (`KismetSystemLibrary.PrintString` "PlayerController: BeginPlay" true true (struct :`G` 0.66 :`B` 1.0 :`A` 1.0) 4.0)
  (`|ExecutionSequence`
    (:`then_0`
      (`self.SetVirtualJoystickVisibility` false))
    (:`then_1`
      (`self.EnableTapRaycast`))))

(event `Key|LeftMouseButton`
  (params (Key :type "Key Structure"))
  (bind (_locationx _locationy) (`WidgetLayoutLibrary.GetMousePositionScaledByDPI` (`GameplayStatics.GetPlayerController` 0)))
  ;[1 1 1] マウス用インプットシステム
  (:`Pressed`
    (if (not (`/Game/LabyrinthCore/Blueprints/Library/BPFL_Labyrinth.IsRunningOnMobile`))
      (`self.OnPress` (`KismetMathLibrary.MakeVector` _locationx _locationy))))
  (:`Released`
    (if (not (`/Game/LabyrinthCore/Blueprints/Library/BPFL_Labyrinth.IsRunningOnMobile`))
      (`self.OnRelease` "Touch1"))))

(event `Key|RightMouseButton`
  (params (Key :type "Key Structure"))
  (bind (_locationx _locationy) (`WidgetLayoutLibrary.GetMousePositionScaledByDPI` (`GameplayStatics.GetPlayerController` 0)))
  ;[1 1 1] マウス用インプットシステム
  (:`Pressed`
    (if (not (`/Game/LabyrinthCore/Blueprints/Library/BPFL_Labyrinth.IsRunningOnMobile`))
      (`self.OnPress` (`KismetMathLibrary.MakeVector` _locationx _locationy) "Touch2")))
  (:`Released`
    (if (not (`/Game/LabyrinthCore/Blueprints/Library/BPFL_Labyrinth.IsRunningOnMobile`))
      (`self.OnRelease` "Touch2"))))

(event `InputAxis|MouseWheel`
  (params (AxisValue :type "Float (single-precision)"))
  (bind _returnvalue (+ (`self.TwoFingerLength`) (* AxisValue 150.0)))
  ;[1 1 1] マウス用インプットシステム
  (if (not (`/Game/LabyrinthCore/Blueprints/Library/BPFL_Labyrinth.IsRunningOnMobile`))
    (if (!= AxisValue 0.0)
      (set `self.TwoFingerDeltaLength` (- (`self.TwoFingerLength`) _returnvalue))
      (set `self.TwoFingerLength` _returnvalue)
      (`self.Pinch`))))

(event `InputAxis|MouseX`
  (params (AxisValue :type "Float (single-precision)"))
  (bind (_locationx _locationy) (`WidgetLayoutLibrary.GetMousePositionScaledByDPI` (`GameplayStatics.GetPlayerController` 0)))
  ;[1 1 1] マウス用インプットシステム
  (if (not (`/Game/LabyrinthCore/Blueprints/Library/BPFL_Labyrinth.IsRunningOnMobile`))
    (if (!= AxisValue 0.0)
      (if (`|EnumInequality` (`.InputState_2_ED25E83C4EAAE7C4AE349192438E6B6A` (break `/Game/LabyrinthCore/Blueprints/Types/FInputData` (`|GetArrayItem` (`self.InputData`)))) "NewEnumerator1")
        (`self.OnMove` "Touch1" (`KismetMathLibrary.MakeVector` _locationx _locationy))))))

(event `InputAxis|MouseY`
  (params (AxisValue :type "Float (single-precision)"))
  (bind (_locationx _locationy) (`WidgetLayoutLibrary.GetMousePositionScaledByDPI` (`GameplayStatics.GetPlayerController` 0)))
  ;[1 1 1] マウス用インプットシステム
  (if (not (`/Game/LabyrinthCore/Blueprints/Library/BPFL_Labyrinth.IsRunningOnMobile`))
    (if (!= AxisValue 0.0)
      (if (`|EnumInequality` (`.InputState_2_ED25E83C4EAAE7C4AE349192438E6B6A` (break `/Game/LabyrinthCore/Blueprints/Types/FInputData` (`|GetArrayItem` (`self.InputData`) 1))) "NewEnumerator1")
        (`self.OnMove` "Touch2" (`KismetMathLibrary.MakeVector` _locationx _locationy))))))

(event `TapRaycast`
  (bind (_worldlocation _worlddirection) (`self.DeprojectScreenPositionToWorld` (.x (* (`self.TapLocation`) (`WidgetLayoutLibrary.GetViewportScale`))) (.y (* (`self.TapLocation`) (`WidgetLayoutLibrary.GetViewportScale`)))))
  ;[1 1 1] タップ処理
  (`/Game/LabyrinthCore/Blueprints/Library/Actor/BPML_PlayerState.LbHasPlayerState` (`/Game/LabyrinthCore/Blueprints/Const/BPCST_PlayerState.PSt_Ingame`)
    (:`true`
      (bind _outhits (`KismetSystemLibrary.LineTraceMulti` _worldlocation (+ _worldlocation (* _worlddirection (`self.RaycastMaxDistance`))) "TraceTypeQuery1" false (`|MakeArray` null :!type "Actor Object Reference")))
      (for _array_element _outhits
        (bind (_bblockinghit _binitialoverlap _time _distance _location _impactpoint _normal _impactnormal _physmat _hitactor) (`GameplayStatics.BreakHitResult` _array_element))
        (bind _asbp_pickup (cast `/Game/LabyrinthCore/Blueprints/BP_Pickup` _hitactor)
          (:`then`
            (bind _pickupcomponent (`/Game/LabyrinthCore/Blueprints/Library/Actor/BPML_PickupComponent.LbGetPlayerPickupComponent`)
              (:`Succeeded`
                (`/Game/LabyrinthCore/Blueprints/PlayerComponents/BP_PickupComponent.ExecutePickup` _pickupcomponent _asbp_pickup)
                (break))))
          (:`CastFailed`
            (bind _asbp_gimmick (cast `/Game/LabyrinthCore/Blueprints/BP_Gimmick` _hitactor)
              (:`then`
                (bind _analyzegimmickcomponent (`/Game/LabyrinthCore/Blueprints/Library/Actor/BPML_GimmickComponent.LbGetAnalyzeGimmickComponent`)
                  (:`Succeeded`
                    (`/Game/LabyrinthCore/Blueprints/PlayerComponents/BP_AnalyzeGimmickComponent.ExecuteGimmick` _analyzegimmickcomponent _asbp_gimmick)
                    (break))))
              (:`CastFailed`
                (`/Game/LabyrinthCore/Blueprints/Library/Actor/BPML_PlayerState.LbIsPlayerState` (`/Game/LabyrinthCore/Blueprints/Const/BPCST_PlayerState.PSt_Ingame_LockMove`)
                  (:`false`
                    (`/Game/LabyrinthCore/Blueprints/Library/Actor/BPML_PlayerMovementComponent.LbPlayerStartMoveRequest` _impactpoint)
                    (break)))))))))))

(event `EnableTapRaycast`
  ;[1 1 1] タップ処理
  (add `self.Tap` (delegate `TapRaycast`)))

(event `DisableTapRaycast`
  ;[1 1 1] タップ処理
  (remove `self.Tap` (delegate `TapRaycast`)))

(event `InputTouch`
  (params (Location :type "Vector Structure") (FingerIndex :type "ETouchIndex Enum"))
  (bind _returnvalue (/ Location (`WidgetLayoutLibrary.GetViewportScale`)))
  ;[1 1 1] タッチ用インプットシステム
  (:`Pressed`
    (`self.OnPress` _returnvalue FingerIndex))
  (:`Released`
    (`self.OnRelease` FingerIndex))
  (:`Moved`
    (`self.OnMove` FingerIndex _returnvalue)))

(fn `AddFingerNum`
  (bind _sessionmaxfingernum (`self.SessionMaxFingerNum`))
  (`|ExecutionSequence`
    (:`then_0`
      (bind _result (`/Engine/EditorBlueprintResources/StandardMacros.IncrementInt` (`self.FingerNum`))
        (:`  `
          (set `self.SessionMaxFingerNum` (`KismetMathLibrary.SelectInt` _result _sessionmaxfingernum (> _result _sessionmaxfingernum))))))
    (:`then_1`
      (return))))

(fn `GetInputData`
  (params (TouchIndex :type Integer))
  (returns (InputData :type "/Game/LabyrinthCore/Blueprints/Types/FInputData Structure"))
  (return (`|GetArrayItem` (`self.InputData`) TouchIndex)))

(fn `OnMove`
  (params (TouchIndex :type "ETouchIndex Enum" :default "Touch1") (Location :type "Vector Structure"))
  (locals (InputTouchIndex :type "ETouchIndex Enum") (TouchLocationArray :type "Array of Vector Structure") (InputLocation :type "Vector Structure") (TouchDeltaLocationArray :type "Array of Vector Structure"))
  (bind _inputdata (`self.InputData`))
  (bind _touchlocationarray (`local.TouchLocationArray`))
  (bind _inputlocation (`local.InputLocation`))
  (bind _touchdeltalocationarray (`local.TouchDeltaLocationArray`))
  (bind _returnvalue (`KismetMathLibrary.Conv_ByteToInt` (`local.InputTouchIndex`)))
  (bind _returnvalue_2 (`KismetMathLibrary.GetVectorArrayAverage` _touchlocationarray))
  (bind (_inputstate _touchlocation _touchdeltalocation _touchstartlocation _pressstarttime) (break `/Game/LabyrinthCore/Blueprints/Types/FInputData` (`|GetArrayItem` _inputdata _returnvalue)))
  (bind (_inputstate_2 _touchlocation_2 _touchdeltalocation_2) (break `/Game/LabyrinthCore/Blueprints/Types/FInputData` (`|GetArrayItem` (`self.InputData`) (`KismetMathLibrary.Conv_ByteToInt` (`local.InputTouchIndex`)))))
  (bind _returnvalue_3 (`KismetMathLibrary.VSize2D` (`KismetMathLibrary.Conv_VectorToVector2D` (- (`|GetArrayItem` _touchlocationarray 1) (`|GetArrayItem` _touchlocationarray)))))
  (set `local.InputTouchIndex` TouchIndex)
  (set `local.InputLocation` Location)
  (`|ExecutionSequence`
    (:`then_0`
      ;[0 0 1] 入力情報の更新
      (if (`|EnumInequality` _inputstate "NewEnumerator1")
        (`KismetArrayLibrary.Array_Set` _inputdata _returnvalue (make `/Game/LabyrinthCore/Blueprints/Types/FInputData` "NewEnumerator2" _inputlocation (- _inputlocation _touchlocation) _touchstartlocation _pressstarttime)) ; 入力情報を登録
      ))
    (:`then_1`
      (switch `int` (`self.FingerNum`)
        (:`1`
          ;[1 1 1] 1本指
          (if (`|EnumInequality` _inputstate_2 "NewEnumerator1")
            (set `self.TouchLocation` _touchlocation_2)
            (set `self.TouchDeltaLocation` _touchdeltalocation_2)
            (`self.Swipe` (`local.InputTouchIndex`))))
        (:`2`
          ;[1 1 1] 2本指
          (if (!= (`KismetMathLibrary.Now`) (`self.TwoFingerLastUpdateTime`))
            (for _array_element (`self.InputData`)
              (bind (_inputstate_3 _touchlocation_3 _touchdeltalocation_3) (break `/Game/LabyrinthCore/Blueprints/Types/FInputData` _array_element))
              (if (`|EnumInequality` _inputstate_3 "NewEnumerator1")
                (bind _returnvalue_4 (`KismetArrayLibrary.Array_Add` (`local.TouchLocationArray`) _touchlocation_3))
                (`KismetArrayLibrary.Array_Add` (`local.TouchDeltaLocationArray`) _touchdeltalocation_3)
                (if (>= _returnvalue_4 1)
                  (break))))
            (if (== (`KismetArrayLibrary.Array_Length` _touchlocationarray) 2)
              (set `self.TwoFingerLastUpdateTime` (`KismetMathLibrary.Now`))
              (`|ExecutionSequence`
                (:`then_0`
                  (set `self.TwoFingerDeltaDot` (`KismetMathLibrary.DotProduct2D` (`KismetMathLibrary.Normal2D` (`KismetMathLibrary.Conv_VectorToVector2D` (`|GetArrayItem` _touchdeltalocationarray 1))) (`KismetMathLibrary.Normal2D` (`KismetMathLibrary.Conv_VectorToVector2D` (`|GetArrayItem` _touchdeltalocationarray))))))
                (:`then_1`
                  (set `self.TwoFingerTouchDeltaLocation` (- _returnvalue_2 (`self.TwoFingerTouchLocation`)))
                  (set `self.TwoFingerTouchLocation` _returnvalue_2)
                  (`self.TwoFingerSwipe`))
                (:`then_2`
                  (set `self.TwoFingerDeltaLength` (- (`self.TwoFingerLength`) _returnvalue_3))
                  (set `self.TwoFingerLength` _returnvalue_3)
                  (`self.Pinch`))))))))))

(fn `OnPress`
  (params (Location :type "Vector Structure") (TouchIndex :type "ETouchIndex Enum" :default "Touch1"))
  (locals (InputTouchIndex :type "ETouchIndex Enum" :default "Touch1") (TouchLocationArray :type "Array of Vector Structure") (InputLocation :type "Vector Structure"))
  (bind _inputlocation (`local.InputLocation`))
  (bind _touchlocationarray (`local.TouchLocationArray`))
  (set `local.InputTouchIndex` TouchIndex)
  (set `local.InputLocation` Location)
  (`|ExecutionSequence`
    (:`then_0`
      ;[0 0 1] 入力情報の更新
      (`KismetArrayLibrary.Array_Set` (`self.InputData`) (`KismetMathLibrary.Conv_ByteToInt` (`local.InputTouchIndex`)) (make `/Game/LabyrinthCore/Blueprints/Types/FInputData` "NewEnumerator0" _inputlocation (0.0 0.0 0.0) _inputlocation (`KismetMathLibrary.Now`))))
    (:`then_1`
      (`self.UpdateFingerNum`) ; 現在のタッチ数を更新
    )
    (:`then_2`
      (switch `int` (`self.FingerNum`)
        (:`1`
          ;[1 1 1] 1本指のときの処理
          (set `self.TouchLocation` (`.TouchLocation_5_855BCCC64584017692B3E789170A3CBC` (break `/Game/LabyrinthCore/Blueprints/Types/FInputData` (`|GetArrayItem` (`self.InputData`) (`KismetMathLibrary.Conv_ByteToInt` (`local.InputTouchIndex`))))))
          (set `self.TouchDeltaLocation` (0.0 0.0 0.0)) ; 移動量は 0 で初期化しておく
          (`self.Pressed` (`local.InputTouchIndex`)))
        (:`2`
          ;[1 1 1] 2本指のときの処理
          (for _array_element (`self.InputData`)
            (bind (_inputstate _touchlocation) (break `/Game/LabyrinthCore/Blueprints/Types/FInputData` _array_element))
            (if (`|EnumInequality` _inputstate "NewEnumerator1")
              (bind _returnvalue (`KismetArrayLibrary.Array_Add` (`local.TouchLocationArray`) _touchlocation))
              (if (>= _returnvalue 1)
                (break))))
          (`|ExecutionSequence`
            (:`then_0`
              (set `self.TwoFingerTouchLocation` (`KismetMathLibrary.GetVectorArrayAverage` _touchlocationarray))
              (set `self.TwoFingerTouchDeltaLocation` (0.0 0.0 0.0)) ; 移動量は 0 で初期化しておく
              (`self.TwoFingerPressed`))
            (:`then_1`
              (set `self.TwoFingerLength` (`KismetMathLibrary.VSize2D` (`KismetMathLibrary.Conv_VectorToVector2D` (- (`|GetArrayItem` _touchlocationarray 1) (`|GetArrayItem` _touchlocationarray)))))
              (set `self.TwoFingerDeltaLength` 0.0))))))))

(fn `OnRelease`
  (params (TouchIndex :type "ETouchIndex Enum" :default "Touch1"))
  (locals (TapLocationArray :type "Array of Vector Structure") (InputTouchIndex :type "ETouchIndex Enum") (PrevFingerNum :type Integer :default 0))
  (bind _inputdata (`self.InputData`))
  (bind _taplocationarray (`local.TapLocationArray`))
  (bind _returnvalue (`KismetMathLibrary.Conv_ByteToInt` (`local.InputTouchIndex`)))
  (bind (_inputstate _touchlocation _touchdeltalocation _touchstartlocation _pressstarttime) (break `/Game/LabyrinthCore/Blueprints/Types/FInputData` (`|GetArrayItem` _inputdata _returnvalue)))
  (set `local.InputTouchIndex` TouchIndex)
  (set `local.PrevFingerNum` (`self.FingerNum`))
  (`|ExecutionSequence`
    (:`then_0`
      (`KismetArrayLibrary.Array_Set` _inputdata _returnvalue (make `/Game/LabyrinthCore/Blueprints/Types/FInputData` "NewEnumerator1" _touchlocation (0.0 0.0 0.0) _touchstartlocation _pressstarttime)))
    (:`then_1`
      (`self.UpdateFingerNum`))
    (:`then_2`
      ;[1 0 0] Release
      (switch `int` (`local.PrevFingerNum`)
        (:`1`
          (`self.Released`))
        (:`2`
          (set `self.TwoFingerDeltaDot` 0.0) ; 離した時に０にしておく
          (`self.TwoFingerReleased`))))
    (:`then_3`
      ;[1 0 0] Tap
      (for _array_element (`self.InputData`)
        (bind (_inputstate_2 _touchlocation_2 _touchdeltalocation_2 _touchstartlocation_2 _pressstarttime_2) (break `/Game/LabyrinthCore/Blueprints/Types/FInputData` _array_element))
        ;;[1 1 1] タップ入力が成功した指をADDする
        (if (and (< (`KismetMathLibrary.GetTotalSeconds` (- (`KismetMathLibrary.Now`) _pressstarttime_2)) (`self.TapJudgeLimitTime`)) (< (`KismetMathLibrary.VSize2D` (- (`KismetMathLibrary.Conv_VectorToVector2D` _touchlocation_2) (`KismetMathLibrary.Conv_VectorToVector2D` _touchstartlocation_2))) (`self.TapJudgeLimitLength`)))
          (`KismetArrayLibrary.Array_Add` (`local.TapLocationArray`) _touchlocation_2)))
      (switch `int` (`KismetArrayLibrary.Array_Length` _taplocationarray) ; ADDした本数によって種類を分ける
        (:`1`
          ;;[1 1 1] 1本指タップ
          (set `self.TapLocation` (`|GetArrayItem` _taplocationarray))
          (`self.Tap`))
        (:`2`
          ;;[1 1 1] 2本指タップ
          (set `self.TwoFingerTapLocation` (`KismetMathLibrary.GetVectorArrayAverage` (`local.TapLocationArray`)))
          (`self.TwoFingerTap`))))))

(fn `SubFingerNum`
  (bind _result (`/Engine/EditorBlueprintResources/StandardMacros.DecrementInt` (`self.FingerNum`))
    (:`  `
      (if (<= _result 0)
        (set `self.SessionMaxFingerNum` 0)))))

(fn `UpdateFingerNum`
  (locals (LocalFingerNum :type Integer))
  (bind _sessionmaxfingernum (`self.SessionMaxFingerNum`))
  ;[1 1 1] 現在のタッチ数を更新
  (for _array_element (`self.InputData`)
    (if (`|EnumInequality` (`.InputState_2_ED25E83C4EAAE7C4AE349192438E6B6A` (break `/Game/LabyrinthCore/Blueprints/Types/FInputData` _array_element)) "NewEnumerator1")
      (`/Engine/EditorBlueprintResources/StandardMacros.IncrementInt` (`local.LocalFingerNum`))))
  (bind _output_get (set `self.FingerNum` (`local.LocalFingerNum`)))
  (if (> _output_get 0)
    (set `self.SessionMaxFingerNum` (`KismetMathLibrary.SelectInt` _output_get _sessionmaxfingernum (> _output_get _sessionmaxfingernum)))
    (else
      (set `self.SessionMaxFingerNum` 0))))

(fn `UserConstructionScript`)