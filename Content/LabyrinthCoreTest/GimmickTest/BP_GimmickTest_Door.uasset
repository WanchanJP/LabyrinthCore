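; Test door gimmick that the player examines and opens by tapping its knob, driven by a GameplayTag state machine (Idle, Open, Opened).
; BeginAnalyze streams in a cutscene sublevel and resumes at Opened if already opened; EndAnalyze unloads it.
; Idle and Opened set their own camera limits and input.
; Open switches the player to cutscene state and plays the sublevel's animation through an interface, moving to Opened on completion.
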(event `self.BeginAnalyze`
  ;[1 0 0] BeginAnalyze
  (`parent.BeginAnalyze`)
  (`/Game/LabyrinthCore/Blueprints/Library/Actor/BPML_Level.LbLoadStreamLevel` (`self.LvN_GimmickTest_Cutscene`) ; カットシーン管理サブレベルをロード
    (:`Completed`
      (`self.ChangeState` (select `bool` (`self.bOpened`) :`false` (`self.St_Idle`) :`true` (`self.St_Opened`))) ; 最初のステートに移行する
    )))

(event `self.EndAnalyze`
  ;[1 0 0] EndAnalyze
  (`parent.EndAnalyze`)
  (`/Game/LabyrinthCore/Blueprints/Library/Actor/BPML_Level.LbUnloadStreamLevel` (`self.LvN_GimmickTest_Cutscene`)) ; カットシーン管理サブレベルをアンロード
  (`self.ChangeState` (`self.St_None`)) ; 終了ステートに移行する
)

(event `self.BeginState`
  ;[0 0 1] BeginState
  (`parent.BeginState`)
  (`|SwitchGameplayTag` (`self.GimmickState`)
    (:`Gimmick.GimmickTest_Door.State.Idle`
      (`self.IdleBegin`))
    (:`Gimmick.GimmickTest_Door.State.Open`
      (`self.OpenBegin`))
    (:`Gimmick.GimmickTest_Door.State.Opened`
      (`self.OpenedBegin`))))

(event `self.EndState`
  ;[0 0 1] EndState
  (`parent.EndState`)
  (`|SwitchGameplayTag` (`self.GimmickState`)
    (:`Gimmick.GimmickTest_Door.State.Idle`
      (`self.IdleEnd`))
    (:`Gimmick.GimmickTest_Door.State.Open`
      (`self.OpenEnd`))
    (:`Gimmick.GimmickTest_Door.State.Opened`
      (`self.OpenedEnd`))))

(event `IdleBegin`
  ;[1 0 0] Begin
  (`|ExecutionSequence`
    (:`then_0`
      ;[1 1 1] このステートで使用する機能を有効化する
      (`self.CameraControlEnable`)
      (`self.BackButtonEnable`)
      (`self.IdleTapEnable`))
    (:`then_1`
      (`self.SetCameraControlParam` (`self.Cam_Idle`)) ; このステートでのカメラ操作範囲を指定する
    )))

(event `IdleEnd`
  ;[1 0 0] End
  ;[1 1 1] このステートで使用した機能を無効化する
  (`self.CameraControlDisable`)
  (`self.BackButtonDisable`)
  (`self.IdleTapDisable`))

(event `IdleTapExec`
  ;[0 0 1] タップ操作
  (`/Game/LabyrinthCore/Blueprints/Library/Actor/BPML_Gimmick.LbIsGimmickPlayable`
    (:`true`
      (bind _outhits (`/Game/LabyrinthCore/Blueprints/Library/Actor/BPML_Gimmick.LbRaycastGimmick`))
      (for _array_element _outhits
        (if (== (`.HitComponent` (`GameplayStatics.BreakHitResult` _array_element)) (`self.CollisionBox_Knob`))
          (`self.ChangeState` (`self.St_Open`))
          (break))))))

(event `IdleTapEnable`
  ;[0 0 1] タップ操作
  (bind _playercontroller (`/Game/LabyrinthCore/Blueprints/Library/Actor/BPML_Player.LbGetPlayerController`)
    (:`Succeeded`
      (add `/Game/LabyrinthCore/Blueprints/BP_PlayerController.Tap` _playercontroller (delegate `IdleTapExec`)))))

(event `IdleTapDisable`
  ;[0 0 1] タップ操作
  (bind _playercontroller (`/Game/LabyrinthCore/Blueprints/Library/Actor/BPML_Player.LbGetPlayerController`)
    (:`Succeeded`
      (remove `/Game/LabyrinthCore/Blueprints/BP_PlayerController.Tap` _playercontroller (delegate `IdleTapExec`)))))

(event `OpenBegin`
  ;[1 0 0] Begin
  (`/Game/LabyrinthCore/Blueprints/Library/Actor/BPML_PlayerState.LbSetPlayerState` (`/Game/LabyrinthCore/Blueprints/Const/BPCST_PlayerState.PSt_Gimmick_Cutscene`)) ; プレイヤーステートを「ギミックのカットシーン」に変更
  (message `/Game/LabyrinthCoreTest/GimmickTest/BPIF_GimmickTest_Door.PlayTestDoorOpen` (`self.Lv_GimmickTest_Cutscene`) self) ; インターフェースを介してアニメーション再生
)

(event `OpenEnd`
  ;[1 0 0] End
  (`/Game/LabyrinthCore/Blueprints/Library/Actor/BPML_PlayerState.LbSetPlayerState` (`/Game/LabyrinthCore/Blueprints/Const/BPCST_PlayerState.PSt_Gimmick_Main`)) ; プレイヤーステートをギミックのメインに変更
)

(event `Open_Cutscene_Finished`
  ;[0 0 1] カットシーンが完了したら呼ばれる
  (set `self.bOpened` true)
  (`self.ChangeState` (`self.St_Opened`)))

(event `OpenedBegin`
  ;[1 0 0] Begin
  (`|ExecutionSequence`
    (:`then_0`
      (`self.CameraControlEnable`)
      (`self.BackButtonEnable`))
    (:`then_1`
      (`self.SetCameraControlParam` (`self.Cam_Opened`)))))

(event `OpenedEnd`
  ;[1 0 0] End
  (`self.CameraControlDisable`)
  (`self.BackButtonDisable`))

(fn `UserConstructionScript`)